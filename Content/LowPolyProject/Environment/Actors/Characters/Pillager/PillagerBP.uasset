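; Pillager character Blueprint that keeps the pillager tethered to its campfire.
; A looping one-second timer replaces Tick and checks the distance to the Campfire.
; When the pillager is alive, has no valid battle reference and strays beyond range, it teleports back onto the campfire, raised by its capsule half-height.
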(event Custom|SlowerTick
  (Utilities|IsValid (Variables|Default|GetCampfire)
    (:Is%20Valid
      (if (> (Math|Vector|VectorLength (- (Transformation|GetActorLocation) (Transformation|GetActorLocation (Variables|Default|GetCampfire)))) 2.5e+03)
        (if (and (not (Variables|Default|GetIsDead)) (not (Utilities|IsValid (Variables|Default|GetBattleRef))))
          (Transformation|SetActorLocation (+ (Transformation|GetActorLocation (Variables|Default|GetCampfire)) (Math|Vector|MakeVector 0.0 0.0 (Variables|/Script/Engine.CapsuleComponent|GetCapsuleHalfHeight (Variables|Default|GetCapsuleComponent)))) false false))))))

(event EventBeginPlay
  (|CallParentFunction)
  (bind _returnvalue (Utilities|Time|SetTimerbyEvent (delegate Custom|SlowerTick) 1.0 true))
  (Variables|Default|SetSlowerTickTimer _returnvalue))

(event Collision|EventActorBeginOverlap
  (params (OtherActor :type Actor%20Object%20Reference))
  (|CallParentFunction OtherActor) ; This node is disabled and will not be called.\nDrag off pins to build functionality.
)

(fn ConstructionScript
  (|CallParentFunction))