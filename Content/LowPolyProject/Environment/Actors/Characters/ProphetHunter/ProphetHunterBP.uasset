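; ProphetHunterBP is the Blueprint for the Prophet Hunter character, extending a parent class with a spawn-in sequence.
; On BeginPlay, after the parent logic, it asks its animation reference to start the "Apparition" action montage with an additional effect.
; A brief delay later, it sets the mesh's skin and clothes materials.
; Tick and construction only call the parent.
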(event EventBeginPlay
  (bind _mesh (Variables|Character|GetMesh))
  (|CallParentFunction)
  ;[1 1 1] Apparition
  (Default|StartActionMontage (Variables|Default|GetAnimationRef) "Apparition" false false false (Utilities|Map|MakeMap "NewEnumerator2" 1.2))
  (Utilities|FlowControl|Delay 0.1)
  (Rendering|Material|SetMaterial _mesh 0 "/Game/LowPolyProject/Environment/Actors/Characters/Human/Peon/Materials/Skin.Skin")
  (Rendering|Material|SetMaterial _mesh 1 "/Game/LowPolyProject/Environment/Actors/Characters/ProphetHunter/Clothes_Inst.Clothes_Inst"))

(event Collision|EventActorBeginOverlap
  (params (OtherActor :type Actor%20Object%20Reference))
  (|CallParentFunction OtherActor) ; This node is disabled and will not be called.\nDrag off pins to build functionality.
)

(event EventTick
  (params (DeltaSeconds :type Float%20%28single-precision%29))
  (|CallParentFunction DeltaSeconds))

(fn ConstructionScript
  (|CallParentFunction))