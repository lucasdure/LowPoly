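; Animal actor Blueprint that registers itself with the animal spawner and unregisters when killed.
; On BeginPlay it retries with a zero delay until the controller's DebugMode reference is valid, then adds itself.
; Both operations edit and write back the spawner's AnimalsSpawned map entry, keyed by the grid step of the animal's current location.
; An ignore flag or missing spawner skips this bookkeeping.
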(event EventBeginPlay
  (|CallParentFunction)
  (Utilities|IsValid (Variables|/Game/LowPolyProject/GameMode/StratController.StratController_C|GetDebugModeRef (Variables|Default|GetControllerRef)) :!label _label
    (:Is%20Valid
      (CallFunction|ChangeSelfReftoAnimalSpawner false))
    (:Is%20Not%20Valid
      (Utilities|FlowControl|Delay 0.0)
      (goto _label))))

(event Collision|EventActorBeginOverlap
  (params (OtherActor :type Actor%20Object%20Reference))
  (|CallParentFunction OtherActor) ; This node is disabled and will not be called.\nDrag off pins to build functionality.
)

(event EventTick
  (params (DeltaSeconds :type Float%20%28single-precision%29))
  (|CallParentFunction DeltaSeconds) ; This node is disabled and will not be called.\nDrag off pins to build functionality.
)

(event EventGetKilledSpecificity
  (CallFunction|ChangeSelfReftoAnimalSpawner true))

(fn ConstructionScript
  (|CallParentFunction))

(fn ChangeSelfReftoAnimalSpawner
  (params (Remove :type Boolean))
  (bind _returnvalue (Transformation|GetActorLocation))
  (bind _controllerref (Variables|Default|GetControllerRef))
  (bind _debugmoderef (Variables|/Game/LowPolyProject/GameMode/StratController.StratController_C|GetDebugModeRef _controllerref))
  (bind _step (Default|GetStepwithCoordinates _debugmoderef _returnvalue))
  (bind _animalspawnerref (Variables|/Game/LowPolyProject/GameMode/DebugMode.DebugMode_C|GetAnimalSpawnerRef _debugmoderef))
  (bind _animalsspawned (Variables|/Game/LowPolyProject/Environment/Actors/Events/AnimalsManagement/AnimalSpawnerBP.AnimalSpawnerBP_C|GetAnimalsSpawned _animalspawnerref))
  (bind _value (Utilities|Map|Find _animalsspawned _step))
  (Utilities|IsValid (Variables|/Game/LowPolyProject/GameMode/DebugMode.DebugMode_C|GetAnimalSpawnerRef (Variables|/Game/LowPolyProject/GameMode/StratController.StratController_C|GetDebugModeRef (Variables|Default|GetControllerRef)))
    (:Is%20Valid
      (if (not (Variables|Default|GetIgnoreRefAddingToAnimalSpawner))
        (if Remove
          (bind _output_get (LocalVariables|SetAnimalListTemp (.animalslist _value)))
          (Utilities|Array|RemoveItem _output_get self)
          (else
            (bind _output_get_2 (LocalVariables|SetAnimalListTemp (.animalslist _value)))
            (Utilities|Array|Add _output_get_2 self)))
        (Utilities|Map|Add _animalsspawned _step (Utilities|Struct|MakeAnimalsRefList (LocalVariables|GetAnimalListTemp)))))))