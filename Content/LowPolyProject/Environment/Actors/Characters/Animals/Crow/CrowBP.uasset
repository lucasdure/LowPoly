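; Crow animal character Blueprint that registers each crow with the game state and makes all crows neutral toward one another.
; On BeginPlay it adds itself to the shared CrowInActions list, then writes mutual Neutral entries in AlreadyMetCharacter with every listed crow, itself included.
; When killed, it runs the parent logic and removes itself from that list.
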(event EventBeginPlay
  (bind _gamestateref (Variables|Default|GetGameStateRef))
  (bind _crowinactions (Variables|/Game/LowPolyProject/GameMode/MyGameState.MyGameState_C|GetCrowInActions _gamestateref))
  (|CallParentFunction)
  ;[1 1 1] Add ref to game state
  (Utilities|Array|Add _crowinactions self)
  (for _array_element _crowinactions
    (Utilities|Map|Add (Variables|Default|GetAlreadyMetCharacter) _array_element (Utilities|Struct|MakeMetCharacters "Neutral"))
    (Utilities|Map|Add (Variables|/Game/LowPolyProject/Environment/Actors/Characters/CharacterBP.CharacterBP_C|GetAlreadyMetCharacter _array_element) self (Utilities|Struct|MakeMetCharacters "Neutral"))))

(event Collision|EventActorBeginOverlap
  (params (OtherActor :type Actor%20Object%20Reference))
  (|CallParentFunction OtherActor) ; This node is disabled and will not be called.\nDrag off pins to build functionality.
)

(event EventTick
  (params (DeltaSeconds :type Float%20%28single-precision%29))
  (|CallParentFunction DeltaSeconds) ; This node is disabled and will not be called.\nDrag off pins to build functionality.
)

(event EventGetKilledSpecificity
  ;[1 1 1] RemoveSelfRef
  (|CallParentFunction)
  (Utilities|Array|RemoveItem (Variables|/Game/LowPolyProject/GameMode/MyGameState.MyGameState_C|GetCrowInActions (Variables|Default|GetGameStateRef)) self))

(fn ConstructionScript
  (|CallParentFunction))