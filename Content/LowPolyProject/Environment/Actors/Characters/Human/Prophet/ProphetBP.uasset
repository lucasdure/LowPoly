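; Prophet human character Blueprint that registers itself with its controller and switches game sound when it enters or leaves battle.
; On BeginPlay it sets itself as the Prophet reference on a valid ControllerRef.
; Each Tick it checks BattleRef validity, using the IsInBattle flag so the GameInstance starts a random battle or base sound only on a state change.
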(event EventBeginPlay
  (|CallParentFunction)
  ;[1 1 1] Set prophet ref in controller
  (Utilities|IsValid (Variables|Default|GetControllerRef)
    (:Is%20Valid
      (Variables|/Game/LowPolyProject/GameMode/StratController.StratController_C|SetProphet (Variables|Default|GetControllerRef) self))))

(event Collision|EventActorBeginOverlap
  (params (OtherActor :type Actor%20Object%20Reference))
  (|CallParentFunction OtherActor) ; This node is disabled and will not be called.\nDrag off pins to build functionality.
)

(event EventTick
  (params (DeltaSeconds :type Float%20%28single-precision%29))
  (bind _gameinstance (Variables|Default|GetGameInstance))
  (|CallParentFunction DeltaSeconds)
  ;[1 1 1] Play Battle Sound
  (Utilities|IsValid (Variables|Default|GetBattleRef)
    (:Is%20Valid
      (if (not (Variables|Default|GetIsInBattle))
        (Variables|Default|SetIsInBattle true)
        (Default|PlayBattleSound _gameinstance 0 true)))
    (:Is%20Not%20Valid
      (if (Variables|Default|GetIsInBattle)
        (Variables|Default|SetIsInBattle false)
        (Default|PlayBaseSound _gameinstance 0 true)))))

(fn ConstructionScript
  (|CallParentFunction))