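; Portal guardian character that keeps a portal inactive until its whole pack has been killed.
; SetPortalToGuard writes the portal to the ActorToKeep blackboard key for the guardian's AI.
; On death, the GetKilledSpecificity event removes the guardian from its PackOfGuardians.
; The last one to die activates the pack's portal and any valid linked portal, then destroys the pack actor.
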(event EventBeginPlay
  (|CallParentFunction))

(event Collision|EventActorBeginOverlap
  (params (OtherActor :type Actor%20Object%20Reference))
  (|CallParentFunction OtherActor) ; This node is disabled and will not be called.\nDrag off pins to build functionality.
)

(event EventTick
  (params (DeltaSeconds :type Float%20%28single-precision%29))
  (|CallParentFunction DeltaSeconds) ; This node is disabled and will not be called.\nDrag off pins to build functionality.
)

(event EventGetKilledSpecificity
  (bind _packofguardians (Variables|Default|GetPackOfGuardians))
  (bind _packofguardians_2 (Variables|Default|GetPackOfGuardians))
  (bind _portal (Variables|/Game/LowPolyProject/Environment/Actors/Characters/PortalGuardians/PacksOfGuardians/PackOfGuardian.PackOfGuardian_C|GetPortal _packofguardians_2))
  (bind _linkedportal (Variables|/Game/LowPolyProject/Environment/Actors/Building/Portals/PortalBP.PortalBP_C|GetLinkedPortal _portal))
  ;[1 1 1] Remove Portal Ref
  (Utilities|IsValid _packofguardians
    (:Is%20Valid
      (Utilities|Array|RemoveItem (Variables|/Game/LowPolyProject/Environment/Actors/Characters/PortalGuardians/PacksOfGuardians/PackOfGuardian.PackOfGuardian_C|GetGuardians _packofguardians) self)
      (if (== (Utilities|Array|Length (Variables|/Game/LowPolyProject/Environment/Actors/Characters/PortalGuardians/PacksOfGuardians/PackOfGuardian.PackOfGuardian_C|GetGuardians (Variables|Default|GetPackOfGuardians))) 0)
        (Default|ActivatePortal _portal)
        (Utilities|IsValid _linkedportal
          (:Is%20Valid
            (Default|ActivatePortal _linkedportal))
          (:Is%20Not%20Valid
            _))
        (Actor|DestroyActor _packofguardians_2)))))

(fn ConstructionScript
  (|CallParentFunction))

(fn SetPortaltoGuard
  (params (PortalToKeep :type Portal%20BP%20Object%20Reference))
  (AI|Components|Blackboard|SetValueasObject (AI|GetBlackboard self) (Utilities|Name|MakeLiteralName "ActorToKeep") PortalToKeep))