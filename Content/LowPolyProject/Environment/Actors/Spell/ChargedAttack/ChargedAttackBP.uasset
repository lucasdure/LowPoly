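; Charged attack spell that hits a line of targets between the caster and the targeted point.
; InitSpell turns and halts the caster, registers as its focused spell, plays the montage and sound, and spawns area and energy-focus particles.
; EndSpell box-detects along that direction, pushes non-casters and deals Intelligence-boosted damage to characters, calling DestroyActor only inside that character branch.
; InterruptSpell removes both particles and destroys the actor.
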(event EventBeginPlay
  (|CallParentFunction) ; This node is disabled and will not be called.\nDrag off pins to build functionality.
)

(event Collision|EventActorBeginOverlap
  (params (OtherActor :type Actor%20Object%20Reference))
  (|CallParentFunction OtherActor) ; This node is disabled and will not be called.\nDrag off pins to build functionality.
)

(event EventTick
  (params (DeltaSeconds :type Float%20%28single-precision%29))
  (|CallParentFunction DeltaSeconds))

(event EventInitSpell
  (params (TargetSpell :type Vector :default "0, 0, 0") (Caster :type Actor%20Object%20Reference) (Target :type Actor%20Object%20Reference))
  (bind _casterref (Variables|Default|GetCasterRef))
  (bind _defaultsceneroot (Variables|Default|GetDefaultSceneRoot))
  (bind _casterref_2 (Variables|Default|GetCasterRef))
  (bind _defaultsceneroot_2 (Variables|Default|GetDefaultSceneRoot))
  (bind _returnvalue (Transformation|GetWorldLocation _defaultsceneroot_2))
  (bind _capsulecomponent (Variables|/Script/Engine.Character|GetCapsuleComponent _casterref_2))
  (bind _capsulehalfheight (Variables|/Script/Engine.CapsuleComponent|GetCapsuleHalfHeight _capsulecomponent))
  (bind _returnvalue_2 (- _returnvalue (Math|Vector|MakeVector 0.0 0.0 _capsulehalfheight)))
  (|CallParentFunction TargetSpell Caster Target)
  (Variables|Default|SetTargetOfSpell TargetSpell)
  (bind _output_get (Variables|Default|SetRotationDirection (Math|Rotator|FindLookatRotation (- (Transformation|GetWorldLocation (Variables|/Script/Engine.Character|GetCapsuleComponent (Variables|Default|GetCasterRef))) (Math|Vector|MakeVector 0.0 0.0 (Variables|/Script/Engine.CapsuleComponent|GetCapsuleHalfHeight (Variables|/Script/Engine.Character|GetCapsuleComponent (Variables|Default|GetCasterRef))))) (Variables|Default|GetTargetOfSpell))))
  (Transformation|SetActorRotation (Variables|Default|GetCasterRef) (Math|Rotator|MakeRotator 0.0 0.0 (.yaw _output_get)))
  (Components|Movement|StopMovementImmediately (Variables|/Script/Engine.Character|GetCharacterMovement _casterref))
  (Default|StartActionMontage (Variables|/Game/LowPolyProject/Environment/Actors/Characters/CharacterBP.CharacterBP_C|GetAnimationRef _casterref) "ChargedAttack" false false false (Utilities|Map|MakeMap))
  (Variables|/Game/LowPolyProject/Environment/Actors/Characters/CharacterBP.CharacterBP_C|SetSpellFocused _casterref self)
  (bind _returnvalue_3 (Effects|SpawnEmitteratLocation "/Game/LowPolyProject/Environment/Particle/RectangleAttackCharge/ChargedAttack1Particle.ChargedAttack1Particle" (+ (/ (- (Variables|Default|GetTargetOfSpell) _returnvalue_2) 2) _returnvalue_2) (Variables|Default|GetRotationDirection) (Math|Conversions|ToVector(Float) (Variables|Default|GetSecondaryCastRange))))
  (Variables|Default|SetParticule1 _returnvalue_3)
  (bind _returnvalue_4 (Effects|SpawnEmitteratLocation "/Game/LowPolyProject/Environment/Particle/Triangles/EnergyFocus.EnergyFocus" (Transformation|GetWorldLocation (Variables|/Script/Engine.Character|GetCapsuleComponent (Variables|Default|GetCasterRef))) (Variables|Default|GetRotationDirection)))
  (Variables|Default|SetParticule2 _returnvalue_4)
  (Audio|SpawnSoundAttached "/Game/LowPolyProject/Environment/Sounds/Voice/ProphetHunter/ProphetHunterLongEffort1.ProphetHunterLongEffort1" _defaultsceneroot "None" (Transformation|GetWorldLocation _defaultsceneroot) "0, 0, 0" "KeepWorldPosition" false 1.0 1.0 0.0 0 0))

(event EventEndSpell
  (bind _secondarycastrange (Variables|Default|GetSecondaryCastRange))
  (bind _rotationdirection (Variables|Default|GetRotationDirection))
  (bind _defaultsceneroot (Variables|Default|GetDefaultSceneRoot))
  (bind _returnvalue (Transformation|GetWorldLocation _defaultsceneroot))
  (bind _returnvalue_2 (Math|Vector|GetForwardVector (Math|Rotator|MakeRotator 0.0 0.0 (.yaw _rotationdirection))))
  (bind _returnvalue_3 (* _returnvalue_2 60000))
  (bind _actorstoreturn (CallFunction|RectDetection (+ (/ (- (Variables|Default|GetTargetOfSpell) _returnvalue) 2) _returnvalue) (Math|Vector|MakeVector (/ _secondarycastrange 2.0) (/ _secondarycastrange 8.0) 5e+01) (Variables|Default|GetRotationDirection)))
  (for _array_element _actorstoreturn
    (if (!= _array_element (Variables|Default|GetCasterRef))
      (CallFunction|PushActor _array_element "NewEnumerator0" _returnvalue_3)
      (bind _ascharacter_bp (Utilities|Casting|CastToCharacterBP _array_element))
      (Class|InteractwithActor|InflictDamagetoActor(Message) _ascharacter_bp (+ (Variables|Default|GetSpellDamages) (+ (Utilities|Struct|BreakCharacterStats (Variables|/Game/LowPolyProject/Environment/Actors/Characters/CharacterBP.CharacterBP_C|GetStats (Variables|Default|GetCasterRef))) (Utilities|Struct|BreakCharacterStats (Utilities|Struct|BreakBuffDebuffStat (Variables|/Game/LowPolyProject/Environment/Actors/Characters/CharacterBP.CharacterBP_C|GetStatBuffList (Variables|Default|GetCasterRef)))))) _returnvalue_3 true "NewEnumerator0" "NewEnumerator2" (Variables|Default|GetCasterRef))
      (Actor|DestroyActor))))

(event EventInterruptSpell
  (Components|DestroyComponent (Variables|Default|GetParticule1))
  (Components|DestroyComponent (Variables|Default|GetParticule2))
  (Actor|DestroyActor))

(fn ConstructionScript
  (|CallParentFunction))