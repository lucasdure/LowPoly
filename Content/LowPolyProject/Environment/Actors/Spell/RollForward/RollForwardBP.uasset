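; RollForwardBP is a spell actor that makes the casting character perform a forward roll toward the target location.
; On InitSpell it casts the caster to CharacterBP and starts a short timed figure on its animation reference, aimed by look-at rotation.
; It attaches a particle effect to the pelvis, plays a roll sound, then destroys itself immediately, leaving the movement to the character's animation reference.
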(event EventBeginPlay
  (|CallParentFunction) ; This node is disabled and will not be called.\nDrag off pins to build functionality.
)

(event Collision|EventActorBeginOverlap
  (params (OtherActor :type Actor%20Object%20Reference))
  (|CallParentFunction OtherActor) ; This node is disabled and will not be called.\nDrag off pins to build functionality.
)

(event EventTick
  (params (DeltaSeconds :type Float%20%28single-precision%29))
  (|CallParentFunction DeltaSeconds) ; This node is disabled and will not be called.\nDrag off pins to build functionality.
)

(event EventInitSpell
  (params (TargetSpell :type Vector :default "0, 0, 0") (Caster :type Actor%20Object%20Reference) (Target :type Actor%20Object%20Reference))
  ;[1 1 1] RollForward
  (|CallParentFunction TargetSpell Caster Target)
  (Variables|Default|SetTargetOfSpell TargetSpell)
  (bind _ascharacter_bp (Utilities|Casting|CastToCharacterBP Caster))
  (bind _output_get (Variables|Default|SetCharacterRef _ascharacter_bp))
  (Default|StartFigure (Variables|/Game/LowPolyProject/Environment/Actors/Characters/CharacterBP.CharacterBP_C|GetAnimationRef _output_get) "NewEnumerator0" 0.8 (Math|Transform|MakeTransform (Variables|Default|GetTargetOfSpell) (Math|Rotator|FindLookatRotation (Transformation|GetWorldLocation (Variables|/Script/Engine.Character|GetCapsuleComponent _output_get)) (Variables|Default|GetTargetOfSpell)) "1,1,1"))
  (Effects|SpawnEmitterAttached "/Game/LowPolyProject/Environment/Particle/Triangles/RollForwardParticle.RollForwardParticle" (Variables|/Script/Engine.Character|GetMesh (Variables|Default|GetCharacterRef)) "Pelvis" (Transformation|GetWorldLocation (Variables|Default|GetDefaultSceneRoot)) (Math|Rotator|MakeRotator 0.0 0.0 (.Yaw (Math|Rotator|BreakRotator (Math|Rotator|FindLookatRotation (Transformation|GetWorldLocation (Variables|/Script/Engine.Character|GetCapsuleComponent _output_get)) (Variables|Default|GetTargetOfSpell))))) "1.000000,1.000000,1.000000" "KeepWorldPosition")
  (Audio|PlaySoundatLocation "/Game/LowPolyProject/Environment/Sounds/Effect/RollForward/RollForward.RollForward" (Transformation|GetWorldLocation (Variables|Default|GetDefaultSceneRoot)) "0, 0, 0" 1.0 1.0 0.0 0 0 0)
  (Actor|DestroyActor))

(fn ConstructionScript
  (|CallParentFunction))