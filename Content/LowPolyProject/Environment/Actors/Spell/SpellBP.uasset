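; Base spell actor that charges its CharacterBP caster mana on start, with empty impact, end and interrupt events.
; Cone and rectangle helpers use box traces, record hits in ThreatenActor to skip repeats, and filter cones by angle.
; Other helpers split targets by cast range or spawn a CollisionSpell for timed cone detection.
; PushActor turns and interrupts characters, or applies force to physics-simulating static meshes.
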(event Custom|InitSpell
  (params (TargetSpell :type Vector) (Caster :type Actor%20Object%20Reference) (Target :type Actor%20Object%20Reference))
  ;[1 1 1] InitSpell
  (bind _ascharacter_bp (Utilities|Casting|CastToCharacterBP Caster)
    (:then
      (bind _output_get (Variables|Default|SetCasterRef _ascharacter_bp))
      (Default|ChangeMana _output_get (* (Variables|Default|GetManaCost) -1) false true)
      (Default|UpdateCharacterPropertiesBase _output_get))
    (:CastFailed
      (Actor|DestroyActor))))

(event Custom|EndSpell)

(event Custom|InterruptSpell)

(event Custom|BaseAttackSpell
  (params (Caster :type Actor%20Object%20Reference) (Target :type Actor%20Object%20Reference))
  ;[1 1 1] BaseAttackSpell
  (bind _ascharacter_bp (Utilities|Casting|CastToCharacterBP Caster)
    (:then
      (bind _output_get (Variables|Default|SetCasterRef _ascharacter_bp))
      (Default|ChangeMana _output_get (* (Variables|Default|GetManaCost) -1) false true)
      (Default|UpdateCharacterPropertiesBase _output_get))
    (:CastFailed
      (Actor|DestroyActor))))

(event Custom|SpellImpact
  (params (TargetImpacted :type Actor%20Object%20Reference)))

(event EventBeginPlay)

(event Collision|EventActorBeginOverlap
  (params (OtherActor :type Actor%20Object%20Reference)))

(event EventTick
  (params (DeltaSeconds :type Float%20%28single-precision%29)))

(fn ConstructionScript)

(fn DetectActorsinCone
  (params (ConeStart :type Vector) (Angle :type Float%20%28single-precision%29) (Direction :type Rotator) (Range :type Float%20%28single-precision%29))
  (bind _targetofspell (Variables|Default|GetTargetOfSpell))
  (bind _returnvalue (Math|Vector|GetForwardVector Direction))
  (bind _returnvalue_2 (- _targetofspell ConeStart))
  (bind _returnvalue_3 (/ _returnvalue_2 2))
  (bind _returnvalue_4 (+ _returnvalue_3 ConeStart))
  (bind _outhits (Class|KismetSystemLibrary|BoxTraceMulti _returnvalue_4 _returnvalue_4 (Math|Vector|MakeVector (/ Range 2.0) (* (Math|Trig|Tan(Degrees) Angle) Range) (/ (Math|Float|Absolute(Float) (- (.Z (Math|Vector|BreakVector ConeStart)) (.z (Variables|Default|GetTargetOfSpell)))) 2.0)) Direction "TraceTypeQuery1" false (Utilities|Array|MakeArray (Variables|Default|GetCasterRef)) "None" true))
  (for _array_element _outhits
    (if (not (Utilities|Set|Contains (LocalVariables|GetThreatenActor) (.hitactor _array_element)))
      (Utilities|Set|Add (LocalVariables|GetThreatenActor) (.hitactor _array_element))
      (if (<= (Class|KismetMathLibrary|DegAcos (Math|Vector|DotProduct (Math|Vector|Normalize (Math|Vector|MakeVector (.x (- (.impactpoint _array_element) ConeStart)) (.y (- (.impactpoint _array_element) ConeStart)) 0.0)) (Math|Vector|Normalize (Math|Vector|MakeVector (.x _returnvalue) (.y _returnvalue) 0.0)))) Angle)
        (Utilities|Array|Add (LocalVariables|GetActorsToReturnLocal) (.hitactor _array_element)))))
  (return (LocalVariables|GetActorsToReturnLocal)))

(fn SeparateConebyDistance
  (params (ConeToSeparate :type Array%20of%20Actor%20Object%20References))
  (for _array_element ConeToSeparate
    (if (< (Math|Vector|VectorLength (Math|Vector|MakeVector (.x (- (Transformation|GetWorldLocation (Variables|Default|GetDefaultSceneRoot)) (Transformation|GetActorLocation _array_element))) (.y (- (Transformation|GetWorldLocation (Variables|Default|GetDefaultSceneRoot)) (Transformation|GetActorLocation _array_element))) 0.0)) (Variables|Default|GetCastRange))
      (Utilities|Array|Add (LocalVariables|GetShortConeLocal) _array_element)
      (else
        (Utilities|Array|Add (LocalVariables|GetLargeTargetLocal) _array_element))))
  (return (LocalVariables|GetShortConeLocal) (LocalVariables|GetLargeTargetLocal)))

(fn PushActor
  (params (Object :type Actor%20Object%20Reference) (InterruptionResponsible :type InterruptionType%20Enum :default "NewEnumerator0") (Force :type Vector))
  (bind _ascharacter_bp (Utilities|Casting|CastToCharacterBP Object)
    (:then
      (Transformation|SetActorRotation _ascharacter_bp (Math|Rotator|MakeRotfromX (* Force -1)))
      (Default|Interrupt (Variables|/Game/LowPolyProject/Environment/Actors/Characters/CharacterBP.CharacterBP_C|GetAnimationRef _ascharacter_bp) InterruptionResponsible (Variables|Default|GetCasterRef) Force))
    (:CastFailed
      (bind _asstatic_mesh_actor (Utilities|Casting|CastToStaticMeshActor Object))
      (if (Physics|IsSimulatingPhysics (Variables|/Script/Engine.StaticMeshActor|GetStaticMeshComponent _asstatic_mesh_actor) "None")
        (Physics|AddForce (Variables|/Script/Engine.StaticMeshActor|GetStaticMeshComponent _asstatic_mesh_actor) Force "None" true)))))

(fn RectDetection
  (params (Position :type Vector) (HalfSize :type Vector) (Direction :type Rotator))
  (bind _outhits (Class|KismetSystemLibrary|BoxTraceMulti Position Position HalfSize Direction "TraceTypeQuery1" false 0 "None" true))
  (for _array_element _outhits
    (if (not (Utilities|Set|Contains (LocalVariables|GetThreatenActor) (.hitactor _array_element)))
      (Utilities|Set|Add (LocalVariables|GetThreatenActor) (.hitactor _array_element))
      (Utilities|Array|Add (LocalVariables|GetActorsToReturnLocal) (.hitactor _array_element))))
  (return (LocalVariables|GetActorsToReturnLocal)))

(fn ConeDetectionTemporal
  (params (ConeStart :type Vector) (Angle :type Float%20%28single-precision%29) (Direction :type Rotator) (Range :type Float%20%28single-precision%29) (Time :type Float%20%28single-precision%29) (Width :type Float%20%28single-precision%29) (Constant :type Boolean))
  (bind _returnvalue (Game|SpawnActorfromClass "/Game/LowPolyProject/Environment/Actors/Spell/CollisionSpell.CollisionSpell_C" (Math|Transform|MakeTransform ConeStart Direction "1,1,1") "AlwaysSpawn" 0 0))
  (Variables|/Game/LowPolyProject/Environment/Actors/Spell/CollisionSpell.CollisionSpell_C|SetAngle _returnvalue Angle)
  (Variables|/Game/LowPolyProject/Environment/Actors/Spell/CollisionSpell.CollisionSpell_C|SetRange _returnvalue Range)
  (Variables|/Game/LowPolyProject/Environment/Actors/Spell/CollisionSpell.CollisionSpell_C|SetTime _returnvalue Time)
  (Variables|/Game/LowPolyProject/Environment/Actors/Spell/CollisionSpell.CollisionSpell_C|SetWidth _returnvalue Width)
  (Variables|/Game/LowPolyProject/Environment/Actors/Spell/CollisionSpell.CollisionSpell_C|SetSpellRef _returnvalue self)
  (Variables|/Game/LowPolyProject/Environment/Actors/Spell/CollisionSpell.CollisionSpell_C|SetConstant _returnvalue Constant)
  (Default|Start _returnvalue))