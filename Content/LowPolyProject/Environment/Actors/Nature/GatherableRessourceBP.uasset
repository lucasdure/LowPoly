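; Gatherable resource actor for the strategy game that can be aimed at, selected in the HUD and harvested by characters.
; It stands in for an instance from a resource pack, re-adding itself to the matching instanced mesh when de-aimed, otherwise toggling a custom-depth highlight.
; Interacting starts the character's extraction animation and moves them into position.
; Helpers convert between amount and scale and remove the resource.
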(event EventBeginPlay
  ;[1 1 1] SetControllerRef
  (bind _asstrat_controller (Utilities|Casting|CastToStratController (Game|GetPlayerController 0)))
  (Variables|Default|SetControllerRef _asstrat_controller))

(event Collision|EventActorBeginOverlap
  (params (OtherActor :type Actor%20Object%20Reference)))

(event EventTick
  (params (DeltaSeconds :type Float%20%28single-precision%29)))

(event EventAimActor
  (params (Aim :type Boolean) (Force :type Boolean) (InstanceIndex :type Integer) (CameraPawnRef :type Camera%20Pawn%20Object%20Reference) (ComponentAimed :type Primitive%20Component%20Object%20Reference))
  (bind _staticmeshcomponent (Variables|Debug|GetStaticMeshComponent))
  (bind _originalpackwhenselected (Variables|Default|GetOriginalPackWhenSelected))
  ;[1 1 1] Change aim color
  (if (or Force (not (Variables|Default|GetIsSelected)))
    (Utilities|IsValid _originalpackwhenselected
      (:Is%20Valid
        (if (not Aim)
          (Class|InstancedStaticMeshComponent|AddInstanceWorldSpace (CallFunction|FindSelfHierarchicalMesh _originalpackwhenselected) (Transformation|GetWorldTransform (Variables|Debug|GetStaticMeshComponent)))
          (Utilities|Array|RemoveItem (Variables|/Game/LowPolyProject/Environment/Actors/Nature/PackOfGatherableRessources.PackOfGatherableRessources_C|GetUninstanciedGatherableRessource _originalpackwhenselected) self)
          (Actor|DestroyActor)))
      (:Is%20Not%20Valid
        (Rendering|SetCustomDepthStencilValue _staticmeshcomponent 3)
        (Rendering|SetRenderCustomDepth _staticmeshcomponent Aim)))))

(event EventSelect/UnselectActor
  (params (Select :type Boolean))
  ;[1 1 1] Select Character
  (CallFunction|AimActor Select true)
  (bind _output_get (Variables|Default|SetIsSelected Select))
  (Default|UpdatePropertiesOfTable (Variables|/Game/LowPolyProject/GameMode/StratController.StratController_C|GetStratHudRef (Variables|Default|GetControllerRef)) (not _output_get) "NewEnumerator2" self))

(event EventPrepareCharacterInterraction
  ;[1 1 1] ExtractRessourceManually
  (Variables|Default|SetOriginalPackWhenSelected 0))

(event EventCharacterInterractwithActor
  (params (CharacterRef :type Character%20BP%20Object%20Reference))
  (bind _self self)
  (bind (_location _rotation) (Default|FindLocationRotationtoCollectRessource CharacterRef _self))
  ;[1 1 1] ExtractRessourceManually
  (if (Default|HasStufftoGatherRessource CharacterRef self)
    (Default|StartExtractRessource (Variables|/Game/LowPolyProject/Environment/Actors/Characters/CharacterBP.CharacterBP_C|GetAnimationRef CharacterRef) _self)
    (Components|MoveComponentTo (Variables|/Script/Engine.Character|GetCapsuleComponent CharacterRef) _location _rotation false false 0.2 false)))

(fn ConstructionScript)

(fn SetRessourceScaleorValue
  (params (Scale :type Vector) (FuturValue :type Integer) (ScaleToValue :type Boolean))
  (bind _returnvalue (Math|Conversions|ToFloat(Integer) FuturValue))
  (bind _maxamount (Variables|Default|GetMaxAmount))
  (bind _minsize (Variables|Default|GetMinSize))
  (bind _minamount (Variables|Default|GetMinAmount))
  (bind _minamount_2 (Variables|Default|GetMinAmount))
  (bind _minsize_2 (Variables|Default|GetMinSize))
  (bind _maxsize (Variables|Default|GetMaxSize))
  (bind _maxamount_2 (Variables|Default|GetMaxAmount))
  (bind _maxsize_2 (Variables|Default|GetMaxSize))
  (bind _returnvalue_2 (Math|Conversions|ToFloat(Integer) _maxamount_2))
  (bind _returnvalue_3 (- _maxsize _minsize))
  (bind _returnvalue_4 (- _maxamount _minamount))
  (bind _returnvalue_5 (Math|Conversions|ToFloat(Integer) _returnvalue_4))
  (bind _returnvalue_6 (/ _returnvalue_3 _returnvalue_5))
  (bind _returnvalue_7 (* _minamount_2 _returnvalue_6))
  (bind _returnvalue_8 (- _minsize_2 _returnvalue_7))
  (bind _returnvalue_9 (Math|Float|MapRangeClamped _returnvalue 0.0 _returnvalue_2 _returnvalue_8 _maxsize_2))
  ;[1 1 1] Set ressource size
  (if ScaleToValue
    (Variables|Default|SetAmount (Math|Float|Round (Math|Float|MapRangeClamped (.x Scale) _returnvalue_8 _maxsize_2 0.0 _returnvalue_2)))
    (else
      (Transformation|SetWorldScale3D (Variables|Debug|GetStaticMeshComponent) (Math|Vector|MakeVector _returnvalue_9 _returnvalue_9 _returnvalue_9)))))

(fn RemoveRessources
  (bind _originalpackwhengathered (Variables|Default|GetOriginalPackWhenGathered))
  (if (Variables|Default|GetIsSelected)
    (Default|UpdatePropertiesOfTable (Variables|/Game/LowPolyProject/GameMode/StratController.StratController_C|GetStratHudRef (Variables|Default|GetControllerRef)) true "NewEnumerator0"))
  (Utilities|IsValid _originalpackwhengathered
    (:Is%20Valid
      (Utilities|Array|RemoveItem (Variables|/Game/LowPolyProject/Environment/Actors/Nature/PackOfGatherableRessources.PackOfGatherableRessources_C|GetUninstanciedGatherableRessource _originalpackwhengathered) self))
    (:Is%20Not%20Valid
      _))
  (Actor|DestroyActor))

(fn FindSelfHierarchicalMesh
  (params (PackConcerned :type Pack%20Of%20Gatherable%20Ressources%20Object%20Reference))
  (return (Utilities|Array|Get(acopy) (Variables|/Game/LowPolyProject/Environment/Actors/Nature/PackOfGatherableRessources.PackOfGatherableRessources_C|GetListOfInstancedMesh PackConcerned) (Utilities|Array|FindItem (Variables|/Game/LowPolyProject/Environment/Actors/Nature/PackOfGatherableRessources.PackOfGatherableRessources_C|GetUsedRessources PackConcerned) (Utilities|GetClass self)))))