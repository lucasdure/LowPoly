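; WindBP is a weather event actor that moves a wind particle system along a randomly chosen path, then removes itself.
; On BeginPlay a random integer selects one of four position timelines, though RandomInteger(3) never reaches the fourth.
; Each timeline feeds a MoveAndDestroyParticle macro that sets the particle system's relative location on update and destroys the actor on finish.
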(event EventBeginPlay
  (switch int (Math|Random|RandomInteger 3)
    (:0
      (bind _position (Timeline|Movement0 PlayFromStart)
        (:Update
          (Utilities|MoveandDestroyParticle _position :!label _label))
        (:Finished
          (goto _label End))))
    (:1
      (bind _position_2 (Timeline|Movement1 PlayFromStart)
        (:Update
          (Utilities|MoveandDestroyParticle _position_2 :!label _label_2))
        (:Finished
          (goto _label_2 End))))
    (:2
      (bind _position_3 (Timeline|Timeline2 PlayFromStart)
        (:Update
          (Utilities|MoveandDestroyParticle _position_3 :!label _label_3))
        (:Finished
          (goto _label_3 End))))
    (:3
      (bind _position_4 (Timeline|Timeline3 PlayFromStart)
        (:Update
          (Utilities|MoveandDestroyParticle _position_4 :!label _label_4))
        (:Finished
          (goto _label_4 End))))))

(event Collision|EventActorBeginOverlap
  (params (OtherActor :type Actor%20Object%20Reference)))

(event EventTick
  (params (DeltaSeconds :type Float%20%28single-precision%29)))

(fn ConstructionScript)