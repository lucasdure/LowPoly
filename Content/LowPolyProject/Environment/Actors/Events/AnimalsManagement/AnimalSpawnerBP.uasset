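; Animal spawner that keeps generation steps -2 to 0 populated with animals while the game mode allows generation.
; On BeginPlay it registers itself with the DebugMode game mode and starts a looping five-second timer.
; Each check tops every step's AnimalsSpawned list up toward ten by asking the game mode to generate random classes from that step's AnimalsSpawnable list, falling back to step 0's list.
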(event EventBeginPlay
  (Utilities|FlowControl|Sequence
    (:then_0
      ;[1 1 1] GameModeRef
      (bind _asdebug_mode (Utilities|Casting|CastToDebugMode (Game|GetGameMode)))
      (bind _output_get (Variables|Default|SetGameModeRef _asdebug_mode))
      (Variables|/Game/LowPolyProject/GameMode/DebugMode.DebugMode_C|SetAnimalSpawnerRef _output_get self))
    (:then_1
      ;[1 1 1] SpawnTimer
      (bind _returnvalue (Utilities|Time|SetTimerbyFunctionName 0 "ShouldSpawnAnimals" 5.0 true))
      (Variables|Default|SetSpawnTimer _returnvalue))))

(event Collision|EventActorBeginOverlap
  (params (OtherActor :type Actor%20Object%20Reference)))

(event EventTick
  (params (DeltaSeconds :type Float%20%28single-precision%29)))

(fn ConstructionScript)

(fn ShouldSpawnAnimals
  (if (Variables|/Game/LowPolyProject/GameMode/DebugMode.DebugMode_C|GetAutoriseGeneration (Variables|Default|GetGameModeRef))
    (for _index (range -2 0)
      (LocalVariables|SetStep _index)
      (if (.ReturnValue (Utilities|Map|Find (Variables|Default|GetAnimalsSpawned) _index))
        _
        (else
          (Utilities|Map|Add :TargetMap (Variables|Default|GetAnimalsSpawned) :Key (LocalVariables|GetStep))))
      (for _index_2 (range 1 (- 10 (Utilities|Array|Length (.animalslist (.Value (Utilities|Map|Find (Variables|Default|GetAnimalsSpawned) _index))))))
        (Default|GenerateOneActorinStep (Variables|Default|GetGameModeRef) (Utilities|Array|Get(acopy) (.animalslist (.Value (Utilities|Map|Find (Variables|Default|GetAnimalsSpawnable) (select (.ReturnValue (Utilities|Map|Find (Variables|Default|GetAnimalsSpawnable) (LocalVariables|GetStep))) (LocalVariables|GetStep) 0)))) (Math|Random|RandomInteger (Utilities|Array|Length (.animalslist (.Value (Utilities|Map|Find (Variables|Default|GetAnimalsSpawnable) (select (.ReturnValue (Utilities|Map|Find (Variables|Default|GetAnimalsSpawnable) (LocalVariables|GetStep))) (LocalVariables|GetStep) 0))))))) (LocalVariables|GetStep) false false)))))