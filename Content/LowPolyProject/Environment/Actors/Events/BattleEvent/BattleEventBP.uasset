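; Battle event actor that marks a circular fight zone and groups the characters inside it into allied teams.
; On spawn it merges into any overlapping battle, enlarging and shifting that one as needed, or registers in GameState and sphere-traces for units.
; Joining characters, including later overlaps, get fight priority, bubble and animation; IsBattleEmpty removes battles with under two populated teams.
; Instanced meshes draw the boundary, and a widget faces and scales with the camera.
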(event OnComponentBeginOverlap(Sphere)
  (params (OverlappedComponent :type Primitive%20Component%20Object%20Reference) (OtherActor :type Actor%20Object%20Reference) (OtherComp :type Primitive%20Component%20Object%20Reference) (OtherBodyIndex :type Integer) (bFromSweep :type Boolean) (SweepResult :type Hit%20Result%20Structure%20%28by%20ref%29))
  ;[1 1 1] BattleStart
  (CallFunction|AddCharacterinBattle OtherActor)
  (Development|PrintString (Utilities|GetDisplayName OtherActor)))

(event Custom|RefreshUnitsInBattle
  (bind _returnvalue (Transformation|GetActorLocation))
  ;[1 1 1] BattleStart
  (bind _outhits (Collision|MultiSphereTraceForObjects _returnvalue _returnvalue (Variables|Default|GetBattleSize) (Utilities|Array|MakeArray "ObjectTypeQuery3") false 0 "None"))
  (for _array_element _outhits
    (CallFunction|AddCharacterinBattle (.hitactor _array_element))))

(event EventBeginPlay
  (bind _returnvalue (Transformation|GetActorLocation))
  ;[1 1 1] Set game state ref
  (bind _asmy_game_state (Utilities|Casting|CastToMyGameState (Game|GetGameState)))
  (Variables|Default|SetGameState _asmy_game_state)
  ;[1 1 1] Clean battle event or not
  (bind _battlefindedreturn (CallFunction|FindNearBattleandReplaceIt))
  (Utilities|IsValid _battlefindedreturn
    (:Is%20Valid
      (CallFunction|RemoveBattle))
    (:Is%20Not%20Valid
      (Utilities|FlowControl|Sequence
        (:then_0
          ;[1 1 1] Add ref to game state
          (Utilities|Array|Add (Variables|/Game/LowPolyProject/GameMode/MyGameState.MyGameState_C|GetBattleList (Variables|Default|GetGameState)) self))
        (:then_1
          ;[1 1 1] BattleStart
          (bind _outhits (Collision|MultiSphereTraceForObjects _returnvalue _returnvalue (Variables|Default|GetBattleSize) (Utilities|Array|MakeArray "ObjectTypeQuery3") false 0 "None"))
          (for _array_element _outhits
            (CallFunction|AddCharacterinBattle (.hitactor _array_element))))))))

(event Collision|EventActorBeginOverlap
  (params (OtherActor :type Actor%20Object%20Reference)))

(event EventTick
  (params (DeltaSeconds :type Float%20%28single-precision%29))
  (bind _widget (Variables|Default|GetWidget))
  (Utilities|FlowControl|Sequence
    (:then_0
      ;[1 1 1] SetPositionOfIndicator
      (CallFunction|SetRotation _widget)
      (CallFunction|SetScale _widget))))

(fn ConstructionScript
  (Components|Sphere|SetSphereRadius (Variables|Default|GetSphere) (Variables|Default|GetBattleSize) true)
  (CallFunction|UpdateLimit))

(fn SetRotation
  (params (WidgetRef :type Scene%20Component%20Object%20Reference))
  (if (Rendering|IsVisible WidgetRef)
    (Transformation|SetWorldRotation WidgetRef (Math|Rotator|MakeRotfromX (* (Transformation|GetActorForwardVector (Game|GetPlayerCameraManager 0)) -1)) false false)))

(fn SetScale
  (params (WidgetRef :type Scene%20Component%20Object%20Reference))
  (bind _returnvalue (Game|GetPlayerCameraManager 0))
  (bind _defaultsceneroot (Variables|Default|GetDefaultSceneRoot))
  (bind _returnvalue_2 (Camera|GetCameraLocation _returnvalue))
  (bind _returnvalue_3 (Transformation|GetWorldLocation _defaultsceneroot))
  (bind _returnvalue_4 (- _returnvalue_2 _returnvalue_3))
  (bind _returnvalue_5 (Math|Vector|VectorLength _returnvalue_4))
  (if (Rendering|IsVisible WidgetRef)
    (Transformation|SetRelativeLocation WidgetRef (Math|Vector|MakeVector 0.0 0.0 (Math|Float|MapRangeClamped _returnvalue_5 3e+02 4e+03 2e+02 1e+03)) false false)
    (Transformation|SetWorldScale3D WidgetRef (* "1.000000,1.000000,1.000000" (Math|Float|MapRangeClamped _returnvalue_5 3e+02 4e+03 0.1 1.0)))))

(fn AddCharacterinBattle
  (params (CharacterToAdd :type Actor%20Object%20Reference))
  (bind _ascharacter_bp (Utilities|Casting|CastToCharacterBP CharacterToAdd))
  (bind _output_get (LocalVariables|SetCharacterToAddLocal _ascharacter_bp))
  (if (and (not (Utilities|IsValid (Variables|/Game/LowPolyProject/Environment/Actors/Characters/CharacterBP.CharacterBP_C|GetBattleRef _output_get))) (not (Variables|/Game/LowPolyProject/Environment/Actors/Characters/CharacterBP.CharacterBP_C|GetNeverFight _output_get)))
    (bind (_array_element _array_index) (Utilities|Array|ForEachLoopwithBreak (Variables|Default|GetTeams))
      (:LoopBody
        (if (Default|AreAllies (Utilities|Array|Get(acopy) (.units _array_element)) (LocalVariables|GetCharacterToAddLocal))
          (Utilities|Array|Add (.units (Utilities|Array|Get(acopy) (Variables|Default|GetTeams) _array_index)) (LocalVariables|GetCharacterToAddLocal))
          (CallFunction|SetCharacterFunctionalities (LocalVariables|GetCharacterToAddLocal))
          (Variables|/Game/LowPolyProject/Environment/Actors/Characters/CharacterBP.CharacterBP_C|SetTeamIndex (LocalVariables|GetCharacterToAddLocal) _array_index)
          (return)))
      (:Completed
        (bind _returnvalue (Utilities|Array|Add (Variables|Default|GetTeams) (Utilities|Struct|MakeTeamStruct (Utilities|Array|MakeArray (LocalVariables|GetCharacterToAddLocal)))))
        (CallFunction|SetCharacterFunctionalities (LocalVariables|GetCharacterToAddLocal))
        (Variables|/Game/LowPolyProject/Environment/Actors/Characters/CharacterBP.CharacterBP_C|SetTeamIndex (LocalVariables|GetCharacterToAddLocal) _returnvalue)
        (return)))
    (else
      (return))))

(fn SetCharacterFunctionalities
  (params (CharacterToSet :type Character%20BP%20Object%20Reference))
  (Variables|/Game/LowPolyProject/Environment/Actors/Characters/CharacterBP.CharacterBP_C|SetBattleRef CharacterToSet self)
  (Default|SetPriority CharacterToSet 6 false)
  (Default|SetBubbleMessage (Variables|/Game/LowPolyProject/Environment/Actors/Characters/CharacterBP.CharacterBP_C|GetBubbleRef CharacterToSet) false "NewEnumerator0" "Fight" "" "" "" false)
  (Variables|/Game/LowPolyProject/Environment/Actors/Characters/Human/Peon/PeonAnimationBP.PeonAnimationBP_C|SetAnimationStatus (Variables|/Game/LowPolyProject/Environment/Actors/Characters/CharacterBP.CharacterBP_C|GetAnimationRef CharacterToSet) "NewEnumerator6")
  (return))

(fn FindNearBattleandReplaceIt
  (bind _array_element (Utilities|Array|ForEachLoopwithBreak (Variables|/Game/LowPolyProject/GameMode/MyGameState.MyGameState_C|GetBattleList (Variables|Default|GetGameState)))
    (:LoopBody
      (Utilities|IsValid _array_element
        (:Is%20Valid
          (if (< (Math|Vector|VectorLength (- (Transformation|GetActorLocation _array_element) (Transformation|GetActorLocation))) (+ (Variables|BattleEventBP_C|GetBattleSize _array_element) (Variables|Default|GetBattleSize)))
            (LocalVariables|SetBattleFinded _array_element)
            (if (> (Math|Vector|VectorLength (- (Transformation|GetActorLocation _array_element) (Transformation|GetActorLocation))) (- (Variables|BattleEventBP_C|GetBattleSize _array_element) (Variables|Default|GetBattleSize)))
              (LocalVariables|SetFuturLocation (+ (* (- (Transformation|GetActorLocation) (Transformation|GetActorLocation (LocalVariables|GetBattleFinded))) (/ (Variables|Default|GetBattleSize) (+ (Variables|BattleEventBP_C|GetBattleSize (LocalVariables|GetBattleFinded)) (Variables|Default|GetBattleSize)))) (Transformation|GetActorLocation (LocalVariables|GetBattleFinded))))
              (bind _output_get (Variables|BattleEventBP_C|SetBattleSize (LocalVariables|GetBattleFinded) (+ (/ (Math|Float|Clamp(Float) (+ (Variables|Default|GetBattleSize) (- (Math|Vector|VectorLength (- (Transformation|GetActorLocation) (Transformation|GetActorLocation (LocalVariables|GetBattleFinded)))) (Variables|BattleEventBP_C|GetBattleSize (LocalVariables|GetBattleFinded)))) 0.0 (Variables|Default|GetBattleSize)) 2.0) (Variables|BattleEventBP_C|GetBattleSize (LocalVariables|GetBattleFinded)))))
              (Components|Sphere|SetSphereRadius (Variables|BattleEventBP_C|GetSphere (LocalVariables|GetBattleFinded)) _output_get true)
              (CallFunction|UpdateLimit (LocalVariables|GetBattleFinded))
              (Transformation|SetActorLocation (LocalVariables|GetBattleFinded) (LocalVariables|GetFuturLocation) false false)
              (return (LocalVariables|GetBattleFinded))
              (else
                (return (LocalVariables|GetBattleFinded))))))))
    (:Completed
      (return (LocalVariables|GetBattleFinded)))))

(fn RemoveCharacterfromBattle
  (params (CharacterRef :type Character%20BP%20Object%20Reference))
  (bind _array_index (Utilities|Array|ForEachLoopwithBreak (Variables|Default|GetTeams))
    (:LoopBody
      (if (== _array_index (Variables|/Game/LowPolyProject/Environment/Actors/Characters/CharacterBP.CharacterBP_C|GetTeamIndex CharacterRef))
        (LocalVariables|SetIndexLocal _array_index)
        (Variables|/Game/LowPolyProject/Environment/Actors/Characters/Human/Peon/PeonAnimationBP.PeonAnimationBP_C|SetAnimationStatus (Variables|/Game/LowPolyProject/Environment/Actors/Characters/CharacterBP.CharacterBP_C|GetAnimationRef CharacterRef) "NewEnumerator0")
        (Default|SetBubbleMessage (Variables|/Game/LowPolyProject/Environment/Actors/Characters/CharacterBP.CharacterBP_C|GetBubbleRef CharacterRef) true "NewEnumerator0" "" "" "" "" false)
        (Utilities|Array|RemoveItem (.units (Utilities|Array|Get(acopy) (Variables|Default|GetTeams) (LocalVariables|GetIndexLocal))) CharacterRef)
        (return)))))

(fn GetTeam
  (params (Character1 :type Character%20BP%20Object%20Reference) (Character2 :type Character%20BP%20Object%20Reference))
  (bind _towncenterlinked (Variables|/Game/LowPolyProject/Environment/Actors/Characters/CharacterBP.CharacterBP_C|GetTownCenterLinked Character2))
  (return (or (and (== (Variables|/Game/LowPolyProject/Environment/Actors/Characters/CharacterBP.CharacterBP_C|GetTownCenterLinked Character1) _towncenterlinked) (Utilities|IsValid _towncenterlinked)) (== (Utilities|GetClass Character1) (Utilities|GetClass Character2)))))

(fn UpdateLimit
  (bind _battlesize (Variables|Default|GetBattleSize))
  (bind _battlesize_2 (Variables|Default|GetBattleSize))
  (bind _returnvalue (/ _battlesize_2 1e+01))
  (bind _returnvalue_2 (Math|Float|Round _returnvalue))
  (bind _returnvalue_3 (- _returnvalue_2 1))
  (Components|InstancedStaticMesh|ClearInstances (Variables|Default|GetLimits))
  (for _index (range 0 _returnvalue_3)
    (Class|InstancedStaticMeshComponent|AddInstanceWorldSpace (Variables|Default|GetLimits) (Math|Transform|MakeTransform (+ (Transformation|GetWorldLocation (Variables|Default|GetDefaultSceneRoot)) (Math|Vector|MakeVector (* (Math|Trig|Cos(Radians) (Math|Float|MapRangeClamped (Math|Conversions|ToFloat(Integer) _index) 0.0 (Math|Conversions|ToFloat(Integer) _returnvalue_3) 0.0 (* (Math|Trig|GetPI) 2.0))) _battlesize) (* _battlesize (Math|Trig|Sin(Radians) (Math|Float|MapRangeClamped (Math|Conversions|ToFloat(Integer) _index) 0.0 (Math|Conversions|ToFloat(Integer) _returnvalue_3) 0.0 (* (Math|Trig|GetPI) 2.0)))) 1.0)) (Math|Rotator|MakeRotfromX (Math|Vector|MakeVector (* (Math|Trig|Cos(Radians) (Math|Float|MapRangeClamped (Math|Conversions|ToFloat(Integer) _index) 0.0 (Math|Conversions|ToFloat(Integer) _returnvalue_3) 0.0 (* (Math|Trig|GetPI) 2.0))) _battlesize) (* _battlesize (Math|Trig|Sin(Radians) (Math|Float|MapRangeClamped (Math|Conversions|ToFloat(Integer) _index) 0.0 (Math|Conversions|ToFloat(Integer) _returnvalue_3) 0.0 (* (Math|Trig|GetPI) 2.0)))) 0.0)) "0.100000,0.300000,1.000000"))))

(fn IsBattleEmpty
  (bind _notemptyteamlocal (LocalVariables|GetNotEmptyTeamLocal))
  (for _array_element (Variables|Default|GetTeams)
    (if (> (Utilities|Array|Length (.units _array_element)) 0)
      (Math|Integer|IncrementInt _notemptyteamlocal
        (:%20%20
          (if (== 2 _notemptyteamlocal)
            (return))))))
  (CallFunction|RemoveBattle)
  (return))

(fn RemoveBattle
  (Utilities|Array|RemoveItem (Variables|/Game/LowPolyProject/GameMode/MyGameState.MyGameState_C|GetBattleList (Variables|Default|GetGameState)) self)
  (for _array_element (Variables|Default|GetTeams)
    (for _array_element_2 (.units _array_element)
      (Utilities|IsValid _array_element_2
        (:Is%20Valid
          (CallFunction|RemoveCharacterfromBattle _array_element_2)))))
  (Actor|DestroyActor))

(fn FindCharacterBattle
  (params (CharacterRef :type Character%20BP%20Object%20Reference))
  (for _array_element (Variables|Default|GetTeams)
    (for _array_element_2 (.units _array_element)
      (if (== _array_element_2 CharacterRef)
        (return true))))
  (return false))

(fn FindProphetBattle
  (for _array_element (Variables|Default|GetTeams)
    (for _array_element_2 (.units _array_element)
      (if (Variables|/Game/LowPolyProject/Environment/Actors/Characters/CharacterBP.CharacterBP_C|GetIsProphet _array_element_2)
        (return true))))
  (return false))