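; TooHeavyBP is an encumbrance speed debuff actor that penalizes a character carrying more than its weight limit.
; Its ChangeVariableifNeeded event sets SpeedPercent from the referenced character's MaxWeight minus WeightOnCharacter, scaled down and clamped so it is never positive.
; Tick calls the parent and spins the halo particle system around yaw at a frame-rate-independent rate.
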(event EventBeginPlay
  (|CallParentFunction) ; This node is disabled and will not be called.\nDrag off pins to build functionality.
)

(event Collision|EventActorBeginOverlap
  (params (OtherActor :type Actor%20Object%20Reference))
  (|CallParentFunction OtherActor) ; This node is disabled and will not be called.\nDrag off pins to build functionality.
)

(event EventTick
  (params (DeltaSeconds :type Float%20%28single-precision%29))
  (|CallParentFunction DeltaSeconds)
  ;[1 1 1] RotateHalo
  (Transformation|AddLocalRotation (Variables|Default|GetParticleSystem) (Math|Rotator|MakeRotator 0.0 0.0 (* (Utilities|Time|GetWorldDeltaSeconds) 6e+01)) false false))

(event EventChangeVariableifNeeded
  (bind _characterref (Variables|Default|GetCharacterRef))
  ;[1 1 1] Change speed debuff
  (Variables|Default|SetSpeedPercent (Math|Float|Clamp(Float) (/ (- (Variables|/Game/LowPolyProject/Environment/Actors/Characters/CharacterBP.CharacterBP_C|GetMaxWeight _characterref) (Variables|/Game/LowPolyProject/Environment/Actors/Characters/CharacterBP.CharacterBP_C|GetWeightOnCharacter _characterref)) 1e+01) -1.0 0.0)))

(fn ConstructionScript
  (|CallParentFunction))