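; SpeedBuffBP is a buff actor that changes a character's speed by adjusting the SpeedBuffDebuff field in its StatBuffList.
; It extends parent apply, update and stop events, adding a flat amount plus a percentage of the character's RunSpeed.
; Updating removes the current bonus, calls ChangeVariableIfNeeded, then adds the recalculated one.
; Stopping subtracts the bonus and destroys the actor.
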(event EventBeginPlay)

(event Collision|EventActorBeginOverlap
  (params (OtherActor :type Actor%20Object%20Reference)))

(event EventUpdateBuff
  (bind _speedconstant (Variables|Default|GetSpeedConstant))
  (bind _characterref (Variables|Default|GetCharacterRef))
  (bind _speedpercent (Variables|Default|GetSpeedPercent))
  (bind _characterref_2 (Variables|Default|GetCharacterRef))
  (bind _runspeed (Variables|/Game/LowPolyProject/Environment/Actors/Characters/CharacterBP.CharacterBP_C|GetRunSpeed _characterref_2))
  (bind _statbufflist (Variables|/Game/LowPolyProject/Environment/Actors/Characters/CharacterBP.CharacterBP_C|GetStatBuffList _characterref))
  (bind _speedbuffdebuff (Utilities|Struct|BreakBuffDebuffStat _statbufflist))
  (bind _returnvalue (* _runspeed _speedpercent))
  (bind _returnvalue_2 (+ _speedconstant _returnvalue))
  ;[1 1 1] Update buff speed
  (|CallParentFunction)
  (Utilities|Struct|SetmembersinBuffDebuffStat (Variables|/Game/LowPolyProject/Environment/Actors/Characters/CharacterBP.CharacterBP_C|GetStatBuffList (Variables|Default|GetCharacterRef)) (- _speedbuffdebuff _returnvalue_2))
  (CallFunction|ChangeVariableifNeeded)
  (Utilities|Struct|SetmembersinBuffDebuffStat (Variables|/Game/LowPolyProject/Environment/Actors/Characters/CharacterBP.CharacterBP_C|GetStatBuffList (Variables|Default|GetCharacterRef)) (+ _speedbuffdebuff _returnvalue_2)))

(event EventApplyBuff
  (params (TargetOfBuff :type Actor%20Object%20Reference))
  ;[1 1 1] SpeedBuff
  (|CallParentFunction TargetOfBuff)
  (CallFunction|ChangeVariableifNeeded)
  (Utilities|Struct|SetmembersinBuffDebuffStat (Variables|/Game/LowPolyProject/Environment/Actors/Characters/CharacterBP.CharacterBP_C|GetStatBuffList (Variables|Default|GetCharacterRef)) (+ (+ (Variables|Default|GetSpeedConstant) (* (Variables|/Game/LowPolyProject/Environment/Actors/Characters/CharacterBP.CharacterBP_C|GetRunSpeed (Variables|Default|GetCharacterRef)) (Variables|Default|GetSpeedPercent))) (Utilities|Struct|BreakBuffDebuffStat (Variables|/Game/LowPolyProject/Environment/Actors/Characters/CharacterBP.CharacterBP_C|GetStatBuffList (Variables|Default|GetCharacterRef))))))

(event EventStopBuff
  ;[1 1 1] SpeedBuff
  (|CallParentFunction)
  (Utilities|Struct|SetmembersinBuffDebuffStat (Variables|/Game/LowPolyProject/Environment/Actors/Characters/CharacterBP.CharacterBP_C|GetStatBuffList (Variables|Default|GetCharacterRef)) (- (Utilities|Struct|BreakBuffDebuffStat (Variables|/Game/LowPolyProject/Environment/Actors/Characters/CharacterBP.CharacterBP_C|GetStatBuffList (Variables|Default|GetCharacterRef))) (+ (Variables|Default|GetSpeedConstant) (* (Variables|/Game/LowPolyProject/Environment/Actors/Characters/CharacterBP.CharacterBP_C|GetRunSpeed (Variables|Default|GetCharacterRef)) (Variables|Default|GetSpeedPercent)))))
  (Actor|DestroyActor))

(fn ConstructionScript
  (|CallParentFunction))