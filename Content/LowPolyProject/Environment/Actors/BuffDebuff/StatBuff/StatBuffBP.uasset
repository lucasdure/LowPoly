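; StatBuffBP is a buff actor that raises a character's six core stats through the character's StatBuffList.
; ApplyBuff runs the parent logic and ChangeVariableIfNeeded, then adds flat StatPoint values plus a StatPercent share of base Stats.
; StopBuff subtracts the same formula, recomputed from current Stats rather than a stored amount, then destroys the actor.
; Percentages are rounded after dividing by 100, so that share scales only in whole multiples.
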(event EventBeginPlay
  (|CallParentFunction) ; This node is disabled and will not be called.\nDrag off pins to build functionality.
)

(event Collision|EventActorBeginOverlap
  (params (OtherActor :type Actor%20Object%20Reference))
  (|CallParentFunction OtherActor) ; This node is disabled and will not be called.\nDrag off pins to build functionality.
)

(event EventTick
  (params (DeltaSeconds :type Float%20%28single-precision%29))
  (|CallParentFunction DeltaSeconds) ; This node is disabled and will not be called.\nDrag off pins to build functionality.
)

(event EventApplyBuff
  (params (TargetOfBuff :type Actor%20Object%20Reference))
  (bind _characterref (Variables|Default|GetCharacterRef))
  (bind _statpercent (Variables|Default|GetStatPercent))
  (bind _characterref_2 (Variables|Default|GetCharacterRef))
  (bind _statpoint (Variables|Default|GetStatPoint))
  (bind _statbufflist (Variables|/Game/LowPolyProject/Environment/Actors/Characters/CharacterBP.CharacterBP_C|GetStatBuffList _characterref))
  (bind _stats (Variables|/Game/LowPolyProject/Environment/Actors/Characters/CharacterBP.CharacterBP_C|GetStats _characterref_2))
  (bind _statbuffdebuff (Utilities|Struct|BreakBuffDebuffStat _statbufflist))
  ;[1 1 1] Stat buff
  (|CallParentFunction TargetOfBuff)
  (CallFunction|ChangeVariableifNeeded)
  (Utilities|Struct|SetmembersinBuffDebuffStat (Variables|/Game/LowPolyProject/Environment/Actors/Characters/CharacterBP.CharacterBP_C|GetStatBuffList (Variables|Default|GetCharacterRef)) (Utilities|Struct|MakeCharacterStats (+ (.strength _statbuffdebuff) (+ (.strength _statpoint) (* (.strength _stats) (Math|Float|Round (/ (Math|Conversions|ToFloat(Integer) (.strength _statpercent)) 1e+02))))) (+ (.agility _statbuffdebuff) (+ (.agility _statpoint) (* (.agility _stats) (Math|Float|Round (/ (Math|Conversions|ToFloat(Integer) (.agility _statpercent)) 1e+02))))) (+ (.dexterity _statbuffdebuff) (+ (.dexterity _statpoint) (* (.dexterity _stats) (Math|Float|Round (/ (Math|Conversions|ToFloat(Integer) (.dexterity _statpercent)) 1e+02))))) (+ (.intelligence _statbuffdebuff) (+ (.intelligence _statpoint) (* (.intelligence _stats) (Math|Float|Round (/ (Math|Conversions|ToFloat(Integer) (.intelligence _statpercent)) 1e+02))))) (+ (.stamina _statbuffdebuff) (+ (.stamina _statpoint) (* (.stamina _stats) (Math|Float|Round (/ (Math|Conversions|ToFloat(Integer) (.stamina _statpercent)) 1e+02))))) (+ (.luck _statbuffdebuff) (+ (.luck _statpoint) (* (.luck _stats) (Math|Float|Round (/ (Math|Conversions|ToFloat(Integer) (.luck _statpercent)) 1e+02))))))))

(event EventStopBuff
  (bind _characterref (Variables|Default|GetCharacterRef))
  (bind _statpercent (Variables|Default|GetStatPercent))
  (bind _characterref_2 (Variables|Default|GetCharacterRef))
  (bind _statpoint (Variables|Default|GetStatPoint))
  (bind _statbufflist (Variables|/Game/LowPolyProject/Environment/Actors/Characters/CharacterBP.CharacterBP_C|GetStatBuffList _characterref))
  (bind _stats (Variables|/Game/LowPolyProject/Environment/Actors/Characters/CharacterBP.CharacterBP_C|GetStats _characterref_2))
  (bind _statbuffdebuff (Utilities|Struct|BreakBuffDebuffStat _statbufflist))
  ;[1 1 1] Stat buff
  (|CallParentFunction)
  (Utilities|Struct|SetmembersinBuffDebuffStat (Variables|/Game/LowPolyProject/Environment/Actors/Characters/CharacterBP.CharacterBP_C|GetStatBuffList (Variables|Default|GetCharacterRef)) (Utilities|Struct|MakeCharacterStats (- (.strength _statbuffdebuff) (+ (.strength _statpoint) (* (.strength _stats) (Math|Float|Round (/ (Math|Conversions|ToFloat(Integer) (.strength _statpercent)) 1e+02))))) (- (.agility _statbuffdebuff) (+ (.agility _statpoint) (* (.agility _stats) (Math|Float|Round (/ (Math|Conversions|ToFloat(Integer) (.agility _statpercent)) 1e+02))))) (- (.dexterity _statbuffdebuff) (+ (.dexterity _statpoint) (* (.dexterity _stats) (Math|Float|Round (/ (Math|Conversions|ToFloat(Integer) (.dexterity _statpercent)) 1e+02))))) (- (.intelligence _statbuffdebuff) (+ (.intelligence _statpoint) (* (.intelligence _stats) (Math|Float|Round (/ (Math|Conversions|ToFloat(Integer) (.intelligence _statpercent)) 1e+02))))) (- (.stamina _statbuffdebuff) (+ (.stamina _statpoint) (* (.stamina _stats) (Math|Float|Round (/ (Math|Conversions|ToFloat(Integer) (.stamina _statpercent)) 1e+02))))) (- (.luck _statbuffdebuff) (+ (.luck _statpoint) (* (.luck _stats) (Math|Float|Round (/ (Math|Conversions|ToFloat(Integer) (.luck _statpercent)) 1e+02)))))))
  (Actor|DestroyActor))

(fn ConstructionScript
  (|CallParentFunction))