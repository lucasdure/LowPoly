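; Base actor for buffs and debuffs that attaches itself to a CharacterBP and follows its location every tick.
; ApplyBuff stores the target and registers the instance in that character's BuffList, a map from buff class to an array of active instances.
; StopBuff removes the instance and drops the class key once its array is empty.
; UpdateBuff and ChangeVariableIfNeeded are empty events, with no gameplay effect defined here.
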(event Custom|ApplyBuff
  (params (TargetOfBuff :type Actor%20Object%20Reference))
  (CallFunction|ApplyBuffFunction TargetOfBuff))

(event Custom|StopBuff
  (CallFunction|StopBuffFunction))

(event Custom|UpdateBuff)

(event Custom|ChangeVariableIfNeeded)

(event EventBeginPlay)

(event Collision|EventActorBeginOverlap
  (params (OtherActor :type Actor%20Object%20Reference)))

(event EventTick
  (params (DeltaSeconds :type Float%20%28single-precision%29))
  (Utilities|IsValid (Variables|Default|GetCharacterRef)
    (:Is%20Valid
      ;[1 1 1] FollowCharacter
      (Transformation|SetWorldLocation (Variables|Default|GetDefaultSceneRoot) (Transformation|GetActorLocation (Variables|Default|GetCharacterRef)) false false))))

(fn ConstructionScript)

(fn ApplyBuffFunction
  (params (Object :type Object%20Object%20Reference))
  (bind _self self)
  (bind _returnvalue (Utilities|GetClass _self))
  (bind _ascharacter_bp (Utilities|Casting|CastToCharacterBP Object))
  (bind _output_get (Variables|Default|SetCharacterRef _ascharacter_bp))
  (if (.ReturnValue (Utilities|Map|Find (Variables|/Game/LowPolyProject/Environment/Actors/Characters/CharacterBP.CharacterBP_C|GetBuffList _output_get) (Utilities|GetClass self)))
    (bind _output_get_2 (LocalVariables|SetBuffCharacterListLocal (.bufflist (.Value (Utilities|Map|Find (Variables|/Game/LowPolyProject/Environment/Actors/Characters/CharacterBP.CharacterBP_C|GetBuffList _output_get) (Utilities|GetClass self))))))
    (Utilities|Array|Add _output_get_2 _self)
    (Utilities|Map|Add (Variables|/Game/LowPolyProject/Environment/Actors/Characters/CharacterBP.CharacterBP_C|GetBuffList (Variables|Default|GetCharacterRef)) _returnvalue (Utilities|Struct|MakeBuffDebuffList _output_get_2))
    (else
      (Utilities|Map|Add (Variables|/Game/LowPolyProject/Environment/Actors/Characters/CharacterBP.CharacterBP_C|GetBuffList (Variables|Default|GetCharacterRef)) _returnvalue (Utilities|Struct|MakeBuffDebuffList (Utilities|Array|MakeArray _self))))))

(fn StopBuffFunction
  (bind _self self)
  (bind _self_2 self)
  (bind _self_3 self)
  (bind _characterref (Variables|Default|GetCharacterRef))
  (bind _characterref_2 (Variables|Default|GetCharacterRef))
  (bind _returnvalue (Utilities|GetClass _self_2))
  (bind _returnvalue_2 (Utilities|GetClass _self_3))
  (bind _bufflist (Variables|/Game/LowPolyProject/Environment/Actors/Characters/CharacterBP.CharacterBP_C|GetBuffList _characterref))
  (bind _bufflist_2 (Variables|/Game/LowPolyProject/Environment/Actors/Characters/CharacterBP.CharacterBP_C|GetBuffList _characterref_2))
  (bind (_value _returnvalue_3) (Utilities|Map|Find _bufflist _returnvalue_2))
  (bind _returnvalue_4 (Utilities|Array|FindItem (.bufflist _value) _self))
  (Utilities|IsValid _characterref
    (:Is%20Valid
      (if (and (!= _returnvalue_4 -1) _returnvalue_3)
        (bind _output_get (LocalVariables|SetBuffCharacterLocal (.bufflist _value)))
        (Utilities|Array|RemoveIndex _output_get _returnvalue_4)
        (if (== (Utilities|Array|Length _output_get) 0)
          (Utilities|Map|Remove _bufflist_2 _returnvalue)
          (else
            (Utilities|Map|Add _bufflist_2 _returnvalue (Utilities|Struct|MakeBuffDebuffList _output_get))))))))