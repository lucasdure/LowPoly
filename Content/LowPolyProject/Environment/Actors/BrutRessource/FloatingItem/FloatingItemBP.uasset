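; Dropped resource or item pickup that spins and bobs, highlights through custom depth, and shows on the strategy HUD when selected.
; SetFloatingItem applies class mesh and amount, then launches a physics sphere with a rarity-colored particle until a hit freezes it and reveals the mesh.
; A sphere trace registers it with nearby town centers, announcing items.
; TakeFromGround routes pickups to hands, equipment or bag, frees untaken amounts, and CleanItemIfNeeded destroys emptied pickups.
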(event OnComponentHit(Sphere)
  (params (HitComponent :type Primitive%20Component%20Object%20Reference) (OtherActor :type Actor%20Object%20Reference) (OtherComp :type Primitive%20Component%20Object%20Reference) (NormalImpulse :type Vector :default "0, 0, 0") (Hit :type Hit%20Result%20Structure%20%28by%20ref%29))
  (bind _sphere (Variables|Default|GetSphere))
  (bind _itemparticle (Variables|Default|GetItemParticle))
  ;[1 1 1] Reveal Item when Fall
  (Physics|SetPhysicsLinearVelocity (Variables|Default|GetSphere) "0, 0, 0" false "None")
  (Physics|SetSimulatePhysics _sphere false)
  (Collision|SetCollisionEnabled _sphere "QueryOnly")
  (Rendering|SetVisibility (Variables|Default|GetStaticMesh) true false)
  (Utilities|IsValid _itemparticle
    (:Is%20Valid
      (Components|DestroyComponent _itemparticle))))

(event EventBeginPlay
  (bind _ressourceclass (Variables|Default|GetRessourceClass))
  (bind _staticmesh (Variables|Default|GetStaticMesh))
  (bind _relativelocation (Variables|/Script/Engine.SceneComponent|GetRelativeLocation _staticmesh))
  (Utilities|FlowControl|Sequence
    (:then_0
      ;[1 1 1] SetControllerRef
      (bind _asstrat_controller (Utilities|Casting|CastToStratController (Game|GetPlayerController 0)))
      (Variables|Default|SetControllerRef _asstrat_controller))
    (:then_1
      ;[1 1 1] ContinuousMovement
      (Utilities|FlowControl|Sequence
        (:then_0
          (bind _rotation (Timeline|RotateItem PlayFromStart)
            (:Update
              (Transformation|SetWorldRotation (Variables|Default|GetSphere) (Math|Rotator|MakeRotator 0.0 0.0 (Math|Float|MapRangeClamped _rotation 0.0 1.0 -1.8e+02 1.8e+02)) false false))))
        (:then_1
          (bind _rotation_2 (Timeline|MoveItem PlayFromStart)
            (:Update
              (if (Utilities|IsValidClass (Variables|Default|GetRessourceClass))
                (Transformation|SetRelativeLocation _staticmesh (Math|Vector|MakeVector (.x _relativelocation) (.y _relativelocation) (+ (Math|Float|MapRangeClamped _rotation_2 0.0 1.0 0.0 2e+01) (.Z (Math|Vector|BreakVector (.Location (Math|Transform|BreakTransform (.FloatingOffset (Utilities|GetClassDefaults (Variables|Default|GetRessourceClass))))))))) false false)))))))
    (:then_2
      ;[1 1 1] DefautBagContainers
      (if (Utilities|IsValidClass _ressourceclass)
        (bind _asbagback_bp (Utilities|Casting|CastToBagbackBPClass _ressourceclass))
        (for _index (range 1 (Utilities|GetClassDefaults _asbagback_bp))
          (Utilities|Array|Add :TargetArray (Variables|Default|GetRessourceInBag)))))))

(event Collision|EventActorBeginOverlap
  (params (OtherActor :type Actor%20Object%20Reference)))

(event EventTick
  (params (DeltaSeconds :type Float%20%28single-precision%29)))

(event EventAimActor
  (params (Aim :type Boolean) (Force :type Boolean) (InstanceIndex :type Integer) (CameraPawnRef :type Camera%20Pawn%20Object%20Reference) (ComponentAimed :type Primitive%20Component%20Object%20Reference))
  ;[1 1 1] Change aim color
  (Variables|Default|SetAimed Aim)
  (if (or Force (not (Variables|Default|GetIsSelected)))
    (Rendering|SetCustomDepthStencilValue (Variables|Default|GetStaticMesh) 3)
    (Rendering|SetRenderCustomDepth (Variables|Default|GetStaticMesh) Aim)))

(event EventSelect/UnselectActor
  (params (Select :type Boolean))
  ;[1 1 1] Select Character
  (CallFunction|AimActor Select true)
  (bind _output_get (Variables|Default|SetIsSelected Select))
  (Default|UpdatePropertiesOfTable (Variables|/Game/LowPolyProject/GameMode/StratController.StratController_C|GetStratHudRef (Variables|Default|GetControllerRef)) (not _output_get) "NewEnumerator3" self))

(event EventCharacterInterractwithActor
  (params (CharacterRef :type Character%20BP%20Object%20Reference))
  ;[1 1 1] InterractWithFloatingItem
  (Default|InteractwithFloatingItem CharacterRef self)
  (Default|SetWeight CharacterRef))

(fn ConstructionScript)

(fn SetFloatingItem
  (params (ClassRef :type Brut%20Ressource%20BP%20Class%20Reference) (Amount :type Integer) (RessourceInBag :type Array%20of%20Ressource%20Amount%20Structures))
  (bind _sphere (Variables|Default|GetSphere))
  (bind (_floatingoffset _mainstaticmeshcomponentofactors) (Utilities|GetClassDefaults ClassRef))
  (Variables|Default|SetRessourceInBag RessourceInBag)
  (Components|StaticMesh|SetStaticMesh (Variables|Default|GetStaticMesh) _mainstaticmeshcomponentofactors)
  (Transformation|SetRelativeLocation (Variables|Default|GetStaticMesh) (.Location (Math|Transform|BreakTransform _floatingoffset)) false false)
  (Variables|Default|SetRessourceClass ClassRef)
  (bind _output_get (Variables|Default|SetAmountFloating Amount))
  (Variables|Default|SetFreeAmountFloating _output_get)
  (bind _returnvalue (Effects|SpawnEmitterAttached "/Game/LowPolyProject/Environment/Actors/BrutRessource/FloatingItem/ItemFalling.ItemFalling" _sphere "None" (Transformation|GetWorldLocation _sphere) "0, 0, 0" "1.000000,1.000000,1.000000" "KeepWorldPosition" false))
  (bind _output_get_2 (Variables|Default|SetItemParticle _returnvalue))
  (Effects|Components|ParticleSystem|SetColorParameter _output_get_2 "Color" (Utilities|Select :Index (.RessourceType (Utilities|GetClassDefaults (Variables|Default|GetRessourceClass))) :NewEnumerator0 "(R=1.000000,G=1.000000,B=1.000000,A=1.000000)" :NewEnumerator1 "(R=0.000000,G=0.838629,B=0.968750,A=1.000000)" :NewEnumerator2 "(R=0.231456,G=0.973958,B=0.103521,A=1.000000)" :NewEnumerator3 "(R=0.014078,G=0.154078,B=0.994792,A=1.000000)" :NewEnumerator4 "(R=1.000000,G=0.005986,B=0.864302,A=1.000000)" :NewEnumerator5 "(R=0.973958,G=0.611542,B=0.000000,A=1.000000)" :NewEnumerator6 "(R=1.000000,G=0.998429,B=0.000000,A=1.000000)"))
  (Variables|Default|SetIsSet true)
  (Physics|AddImpulse (Variables|Default|GetSphere) (* (Math|Vector|RotateVector "5.000000,5.000000,20.000000" (Math|Rotator|MakeRotator 0.0 0.0 (Math|Random|RandomFloatinRange -1.8e+02 1.8e+02))) 20) "None" true)
  (CallFunction|WarnPeopleItemAvailable))

(fn FreeAmount
  (params (AmountToFree :type Integer))
  (Variables|Default|SetFreeAmountFloating (+ AmountToFree (Variables|Default|GetFreeAmountFloating)))
  (if (.IsItem (Utilities|GetClassDefaults (Variables|Default|GetRessourceClass)))
    (for _array_element (Variables|Default|GetTownsLinked)
      (Variables|/Game/LowPolyProject/Environment/Actors/Building/TownCenters/TownCenterBP.TownCenterBP_C|SetItemAvailable _array_element true)
      (Default|WarnItemAvailable _array_element)
      (return))
    (else
      (return))))

(fn TakefromGround
  (params (AmountTaken :type Integer) (CharacterWhoTakes :type Character%20BP%20Object%20Reference))
  (LocalVariables|SetAmountTakenLocal (Math|Integer|Clamp(Integer) AmountTaken 1 (Variables|Default|GetAmountFloating)))
  (if (not (Utilities|GetClassDefaults (Variables|Default|GetRessourceClass)))
    _
    (else
      (bind _asitem_bp (Utilities|Casting|CastToItemBPClass (Variables|Default|GetRessourceClass)))
      (bind _output_get (LocalVariables|SetItemClassLocal _asitem_bp))
      (LocalVariables|SetTwoHands (.TwoHands (Utilities|GetClassDefaults _output_get)))
      (switch Utilities|FlowControl|Switch|SwitchonClothType (Utilities|GetClassDefaults _output_get)
        (:NewEnumerator0
          _)
        (:NewEnumerator5
          (if (Utilities|IsValidClass (Variables|/Game/LowPolyProject/Environment/Actors/Characters/CharacterBP.CharacterBP_C|GetBagbackClass CharacterWhoTakes))
            (if (CallFunction|IsBagEmpty)
              (bind _amounttakeninbag (Default|PlaceAutomaticinBag CharacterWhoTakes (Variables|Default|GetRessourceClass) (LocalVariables|GetAmountTakenLocal) false :!label _label))
              (if (== _amounttakeninbag 0)
                (CallFunction|FreeAmount (LocalVariables|GetAmountTakenLocal) :!label _label_2)
                (return 0 false false)
                (else
                  (LocalVariables|SetInBagLocal true)))
              (else
                (goto _label_2))))
          (Variables|Default|SetAmountFloating (- (Variables|Default|GetAmountFloating) (LocalVariables|GetAmountTakenLocal)) :!label _label_3)
          (return (LocalVariables|GetAmountTakenLocal) (LocalVariables|GetInBagLocal) false))
        (:NewEnumerator3
          (if (Utilities|IsValidClass (Variables|/Game/LowPolyProject/Environment/Actors/Characters/CharacterBP.CharacterBP_C|GetHelmetClass CharacterWhoTakes))
            (goto _label)
            (else
              (goto _label_3)))))))
  (bind (_canttake _stackressource _lefthand) (CallFunction|CanTakeIteminHand (LocalVariables|GetTwoHands) CharacterWhoTakes (not (Utilities|GetClassDefaults (Variables|Default|GetRessourceClass)))))
  (if _canttake
    (bind _amounttakeninbag_2 (Default|PlaceAutomaticinBag CharacterWhoTakes (Variables|Default|GetRessourceClass) (LocalVariables|GetAmountTakenLocal) false))
    (if (== _amounttakeninbag_2 0)
      (CallFunction|FreeAmount (LocalVariables|GetAmountTakenLocal))
      (return 0 false false)
      (else
        (LocalVariables|SetInBagLocal true)))
    (else
      (LocalVariables|SetLeftSideLocal _lefthand)
      (CallFunction|FreeAmount (- (LocalVariables|GetAmountTakenLocal) (Math|Integer|Clamp(Integer) (LocalVariables|GetAmountTakenLocal) 0 (- (.MaxAmountInHands (Utilities|GetClassDefaults (Variables|Default|GetRessourceClass))) (Utilities|Struct|BreakRessourceAmount (select _lefthand (Variables|/Game/LowPolyProject/Environment/Actors/Characters/CharacterBP.CharacterBP_C|GetRessourceInHandLeft CharacterWhoTakes) (Variables|/Game/LowPolyProject/Environment/Actors/Characters/CharacterBP.CharacterBP_C|GetRessourceInHandRight CharacterWhoTakes)))))))
      (LocalVariables|SetAmountTakenLocal (Math|Integer|Clamp(Integer) (LocalVariables|GetAmountTakenLocal) 0 (- (.MaxAmountInHands (Utilities|GetClassDefaults (Variables|Default|GetRessourceClass))) (Utilities|Struct|BreakRessourceAmount (select _lefthand (Variables|/Game/LowPolyProject/Environment/Actors/Characters/CharacterBP.CharacterBP_C|GetRessourceInHandLeft CharacterWhoTakes) (Variables|/Game/LowPolyProject/Environment/Actors/Characters/CharacterBP.CharacterBP_C|GetRessourceInHandRight CharacterWhoTakes))))))))
  (Variables|Default|SetAmountFloating (- (Variables|Default|GetAmountFloating) (LocalVariables|GetAmountTakenLocal)))
  (return (LocalVariables|GetAmountTakenLocal) (LocalVariables|GetInBagLocal) (LocalVariables|GetLeftSideLocal)))

(fn CleanItemifNeeded
  (if (<= (Variables|Default|GetAmountFloating) 0)
    (for _array_element (Variables|Default|GetTownsLinked)
      (if (!= (Utilities|Array|FindItem (Variables|/Game/LowPolyProject/Environment/Actors/Building/TownCenters/TownCenterBP.TownCenterBP_C|GetRessourceOnGround _array_element) self) -1)
        (Utilities|Array|RemoveIndex (Variables|/Game/LowPolyProject/Environment/Actors/Building/TownCenters/TownCenterBP.TownCenterBP_C|GetRessourceOnGround _array_element) (Utilities|Array|FindItem (Variables|/Game/LowPolyProject/Environment/Actors/Building/TownCenters/TownCenterBP.TownCenterBP_C|GetRessourceOnGround _array_element) self))))
    (Actor|DestroyActor))
  (return))

(fn CanTakeIteminHand
  (params (ItemIsTwoHand :type Boolean) (CharacterRef :type Character%20BP%20Object%20Reference) (ItemIsRessource :type Boolean))
  (bind _ressourceclass (Variables|Default|GetRessourceClass))
  (bind _ressourceclass_2 (Variables|Default|GetRessourceClass))
  (bind _ressourceclass_3 (Variables|Default|GetRessourceClass))
  (bind _ressourceclass_4 (Variables|Default|GetRessourceClass))
  (bind _tooltocontainit (Utilities|GetClassDefaults _ressourceclass))
  (bind _tooltocontainit_2 (Utilities|GetClassDefaults _ressourceclass_2))
  (bind _ressourceinhandleft (Variables|/Game/LowPolyProject/Environment/Actors/Characters/CharacterBP.CharacterBP_C|GetRessourceInHandLeft CharacterRef))
  (bind _ressourceinhandright (Variables|/Game/LowPolyProject/Environment/Actors/Characters/CharacterBP.CharacterBP_C|GetRessourceInHandRight CharacterRef))
  (bind _ressourcerighthand (Variables|/Game/LowPolyProject/Environment/Actors/Characters/CharacterBP.CharacterBP_C|GetRessourceRightHand CharacterRef))
  (bind _ressourceinhandright_2 (Variables|/Game/LowPolyProject/Environment/Actors/Characters/CharacterBP.CharacterBP_C|GetRessourceInHandRight CharacterRef))
  (bind _ressourceinhandleft_2 (Variables|/Game/LowPolyProject/Environment/Actors/Characters/CharacterBP.CharacterBP_C|GetRessourceInHandLeft CharacterRef))
  (bind (_ressource _amount) (Utilities|Struct|BreakRessourceAmount _ressourceinhandleft_2))
  (bind (_ressource_2 _amount_2) (Utilities|Struct|BreakRessourceAmount _ressourceinhandright_2))
  (bind _returnvalue (Utilities|IsValid _ressourcerighthand))
  (Utilities|IsValid (Variables|/Game/LowPolyProject/Environment/Actors/Characters/CharacterBP.CharacterBP_C|GetRessourceRightHand CharacterRef)
    (:Is%20Valid
      (bind _output_get (LocalVariables|SetRightCannotContainResource (or (not (Utilities|IsValidClass _tooltocontainit)) (!= _tooltocontainit (Utilities|GetClass (Variables|/Game/LowPolyProject/Environment/Actors/Characters/CharacterBP.CharacterBP_C|GetRessourceRightHand CharacterRef))))))
      (if (not _output_get)
        (if (not (Utilities|IsValidClass (.ressource _ressourceinhandleft)))
          (return false false true)
          (elif (< (.amount _ressourceinhandleft) (.MaxAmountInHands (Utilities|GetClassDefaults (.ressource _ressourceinhandleft))))
            (return false false true)
            (else
              _))))
      (if (Variables|/Game/LowPolyProject/Environment/Actors/BrutRessource/BrutRessourceBP.BrutRessourceBP_C|GetTwoHands (Variables|/Game/LowPolyProject/Environment/Actors/Characters/CharacterBP.CharacterBP_C|GetRessourceRightHand CharacterRef))
        (return true false false)
        (else
          _)))
    (:Is%20Not%20Valid
      (LocalVariables|SetRightCannotContainResource true)))
  (Utilities|IsValid (Variables|/Game/LowPolyProject/Environment/Actors/Characters/CharacterBP.CharacterBP_C|GetRessourceLeftHand CharacterRef)
    (:Is%20Valid
      (bind _output_get_2 (LocalVariables|SetLeftCannotContainResource (or (not (Utilities|IsValidClass _tooltocontainit_2)) (!= _tooltocontainit_2 (Utilities|GetClass (Variables|/Game/LowPolyProject/Environment/Actors/Characters/CharacterBP.CharacterBP_C|GetRessourceLeftHand CharacterRef))))))
      (if (not _output_get_2)
        (if (not (Utilities|IsValidClass (.ressource _ressourceinhandright)))
          (return false false false)
          (elif (< (.amount _ressourceinhandright) (.MaxAmountInHands (Utilities|GetClassDefaults (.ressource _ressourceinhandright))))
            (return false false false)
            (else
              _))))
      (if (Variables|/Game/LowPolyProject/Environment/Actors/BrutRessource/BrutRessourceBP.BrutRessourceBP_C|GetTwoHands (Variables|/Game/LowPolyProject/Environment/Actors/Characters/CharacterBP.CharacterBP_C|GetRessourceLeftHand CharacterRef))
        (return true false false)
        (else
          _)))
    (:Is%20Not%20Valid
      (LocalVariables|SetLeftCannotContainResource true)))
  (if (Utilities|IsValidClass (.ToolToContainIt (Utilities|GetClassDefaults (Variables|Default|GetRessourceClass))))
    (return true false false)
    (elif ItemIsRessource
      (if (Utilities|IsValidClass (Utilities|Struct|BreakRessourceAmount (Variables|/Game/LowPolyProject/Environment/Actors/Characters/CharacterBP.CharacterBP_C|GetRessourceInHandRight CharacterRef)))
        (if (and (== _ressource_2 _ressourceclass_4) (< _amount_2 (.MaxAmountInHands (Utilities|GetClassDefaults _ressourceclass_4))))
          (return false true false)
          (elif (Utilities|IsValidClass (Utilities|Struct|BreakRessourceAmount (Variables|/Game/LowPolyProject/Environment/Actors/Characters/CharacterBP.CharacterBP_C|GetRessourceInHandLeft CharacterRef)))
            (if (and (== _ressource _ressourceclass_3) (< _amount (.MaxAmountInHands (Utilities|GetClassDefaults _ressourceclass_3))))
              (return false true true)
              (else
                (return true false true)))
            (else
              (return false false true))))
        (else
          (return false false false)))
      (elif ItemIsTwoHand
        (return (or (Utilities|IsValid (Variables|/Game/LowPolyProject/Environment/Actors/Characters/CharacterBP.CharacterBP_C|GetRessourceRightHand CharacterRef)) (Utilities|IsValid (Variables|/Game/LowPolyProject/Environment/Actors/Characters/CharacterBP.CharacterBP_C|GetRessourceLeftHand CharacterRef))) false false)
        (else
          (return (and _returnvalue (Utilities|IsValid (Variables|/Game/LowPolyProject/Environment/Actors/Characters/CharacterBP.CharacterBP_C|GetRessourceLeftHand CharacterRef))) false _returnvalue))))))

(fn IsBagEmpty
  (for _array_element (Variables|Default|GetRessourceInBag)
    (if (Utilities|IsValidClass (.ressource _array_element))
      (return false)))
  (return true))

(fn CanStackRessource
  (params (Character :type Character%20BP%20Object%20Reference))
  (bind _ressourceinhandleft (Variables|/Game/LowPolyProject/Environment/Actors/Characters/CharacterBP.CharacterBP_C|GetRessourceInHandLeft Character))
  (if (Utilities|IsValidClass (.ressource _ressourceinhandleft))
    (return (and (< (.amount _ressourceinhandleft) (.MaxAmountInHands (Utilities|GetClassDefaults (.ressource _ressourceinhandleft)))) (== (.ressource _ressourceinhandleft) (Variables|Default|GetRessourceClass))))
    (else
      (return false))))

(fn WarnPeopleItemAvailable
  (bind _sphere (Variables|Default|GetSphere))
  (bind _returnvalue (Transformation|GetWorldLocation _sphere))
  (bind _outhits (Collision|MultiSphereTraceForObjects _returnvalue _returnvalue 5e+03 (Utilities|Array|MakeArray "ObjectTypeQuery7") false 0 "None"))
  (for _array_element _outhits
    (if (!= (Utilities|Array|FindItem (Variables|/Script/Engine.Actor|GetTags (.hitactor _array_element)) "TownCenter") -1)
      (bind _astown_center_bp (Utilities|Casting|CastToTownCenterBP (.hitactor _array_element)))
      (Utilities|Array|Add (Variables|/Game/LowPolyProject/Environment/Actors/Building/TownCenters/TownCenterBP.TownCenterBP_C|GetRessourceOnGround _astown_center_bp) self)
      (Utilities|Array|Add (Variables|Default|GetTownsLinked) _astown_center_bp)
      (if (.IsItem (Utilities|GetClassDefaults (Variables|Default|GetRessourceClass)))
        (Variables|/Game/LowPolyProject/Environment/Actors/Building/TownCenters/TownCenterBP.TownCenterBP_C|SetItemAvailable _astown_center_bp true)
        (Default|WarnItemAvailable _astown_center_bp)))))