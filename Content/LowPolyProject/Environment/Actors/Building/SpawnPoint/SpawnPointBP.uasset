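; Spawn point building actor that spawns the Prophet in a meditating state above its PositionProphet marker on BeginPlay.
; A looping one-second timer checks whether the Prophet has strayed too far from the actor and, if so, teleports it back above the marker.
; During that correction, a downward WorldStatic trace, when it hits, first moves the spawn point to the surface and reframes the player camera on it.
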(event Custom|VerifyProphetIsAtGoodPosition
  (bind _positionprophet (Variables|Default|GetPositionProphet))
  (bind _staticmeshcomponent (Variables|Default|GetStaticMeshComponent))
  (bind _returnvalue (Transformation|GetWorldLocation _staticmeshcomponent))
  ;[1 1 1] Correct prophet position
  (if (> (Math|Vector|VectorLength (- (Transformation|GetActorLocation (Variables|Default|GetProphet)) (Transformation|GetActorLocation))) 5e+02)
    (bind (_outhit _returnvalue_2) (Collision|LineTraceForObjects (+ _returnvalue "0, 0,2000.000000") _returnvalue (Utilities|Array|MakeArray "ObjectTypeQuery1") false 0 "ForDuration"))
    (if _returnvalue_2
      (Transformation|SetActorLocationAndRotation (.Location (Collision|BreakHitResult _outhit)) (Transformation|GetActorRotation))
      (Transformation|SetWorldLocationAndRotation (Variables|/Game/LowPolyProject/GameMode/CameraPawn.CameraPawn_C|GetCamera (Variables|/Game/LowPolyProject/GameMode/StratController.StratController_C|GetPlayerPawnRef (Variables|Default|GetControllerRef))) (- (.Location (Collision|BreakHitResult _outhit)) "400.000000, 0,-100.000000") (Math|Rotator|FindLookatRotation (- (.Location (Collision|BreakHitResult _outhit)) "400.000000, 0,-100.000000") (- (.Location (Collision|BreakHitResult _outhit)) "0.000000, 0,-100.000000")) false false))
    (Transformation|SetActorLocationAndRotation (Variables|Default|GetProphet) (+ (Transformation|GetWorldLocation _positionprophet) "0, 0,200.000000") (Transformation|GetWorldRotation _positionprophet))))

(event EventBeginPlay
  (bind _positionprophet (Variables|Default|GetPositionProphet))
  (|CallParentFunction)
  (Utilities|FlowControl|Sequence
    (:then_0
      ;[1 1 1] Spawn prophet
      (bind _returnvalue (Game|SpawnActorfromClass "/Game/LowPolyProject/Environment/Actors/Characters/Human/Prophet/ProphetBP.ProphetBP_C" (Math|Transform|MakeTransform (+ (Transformation|GetWorldLocation _positionprophet) "0, 0,200.000000") (Transformation|GetWorldRotation _positionprophet) "1,1,1") "AdjustIfPossibleButAlwaysSpawn" 0 0))
      (bind _output_get (Variables|Default|SetProphet _returnvalue))
      (Variables|/Game/LowPolyProject/Environment/Actors/Characters/Human/Peon/PeonAnimationBP.PeonAnimationBP_C|SetIsMeditating (Variables|/Game/LowPolyProject/Environment/Actors/Characters/CharacterBP.CharacterBP_C|GetAnimationRef _output_get) true))
    (:then_2
      ;[1 1 1] Correct prophet position
      (bind _returnvalue_2 (Utilities|Time|SetTimerbyEvent (delegate Custom|VerifyProphetIsAtGoodPosition) 1.0 true))
      (Variables|Default|SetProphetCorrectorTimer _returnvalue_2))))

(event Collision|EventActorBeginOverlap
  (params (OtherActor :type Actor%20Object%20Reference))
  (|CallParentFunction OtherActor) ; This node is disabled and will not be called.\nDrag off pins to build functionality.
)

(event EventTick
  (params (DeltaSeconds :type Float%20%28single-precision%29))
  (|CallParentFunction DeltaSeconds) ; This node is disabled and will not be called.\nDrag off pins to build functionality.
)

(fn ConstructionScript
  (|CallParentFunction))