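; Town center actor that procedurally generates a village with a random name, indicator widget, storehouse, granary, houses and other buildings.
; A grid of downward traces keeps flat spots, which are shuffled, overlap-checked and cleared of instanced foliage before buildings spawn facing the center.
; It then spawns inhabitants with an optionally random village color, collects nearby gatherable resource packs, and flags available items or unfamiliar buildings to inhabitants through AI blackboards.
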(event EventBeginPlay
  (bind _returnvalue (Math|Random|RandomFloat))
  (bind _staticmeshcomponent (Variables|Default|GetStaticMeshComponent))
  (bind _returnvalue_2 (* 10000 _returnvalue))
  (bind _returnvalue_3 (Transformation|GetWorldLocation _staticmeshcomponent))
  (bind _returnvalue_4 (Math|Float|Truncate _returnvalue_2))
  (bind _returnvalue_5 (Math|Random|MakeRandomStream _returnvalue_4))
  (bind _returnvalue_6 (Math|Random|RandomFloatfromStream _returnvalue_5))
  (|CallParentFunction)
  (Utilities|FlowControl|Sequence
    (:then_0
      ;[1 1 1] GetTownIndicatorRef
      (bind _astown_indicator (Utilities|Casting|CastToTownIndicator (UserInterface|GetUserWidgetObject (Variables|Default|GetTownIndicator))))
      (bind _output_get (Variables|Default|SetTownIndicatorRef _astown_indicator))
      (Variables|/Game/LowPolyProject/Environment/Hud/Town/TownIndicator.TownIndicator_C|SetTownCenterRef _output_get self)
      ;[1 1 1] GenerateTownName
      (bind _futurname (Default|GeneratesNames (Variables|Default|GetGameStateRef) true))
      (bind _output_get_2 (Variables|Default|SetTownName (Utilities|String|StringToName _futurname)))
      (Rendering|Components|TextRender|SetText (Variables|/Game/LowPolyProject/Environment/Hud/Town/TownIndicator.TownIndicator_C|GetTownNameText (Variables|Default|GetTownIndicatorRef)) (Utilities|Text|ToText(Name) _output_get_2)))
    (:then_1
      ;[1 1 1] Building generation
      (CallFunction|GenerateBuildings))
    (:then_2
      ;[1 1 1] Randomize human color
      (if (Variables|Default|GetRandomizeColor)
        (Variables|Default|SetVillageMainColor (Math|Conversions|ToColor(LinearColor) (Math|Color|MakeColor (Math|Random|RandomFloatfromStream (Math|Random|MakeRandomStream (Math|Float|Truncate (* 10000 _returnvalue_6)))) _returnvalue_6 _returnvalue))))
      ;[1 1 1] Generate livings
      (for _array_element (Variables|Default|GetHabitationCreated)
        (Default|GenerateHabitants _array_element (Variables|/Game/LowPolyProject/Environment/Actors/Building/BuildingBP.BuildingBP_C|GetHabitantInTheBuilding _array_element) false (Variables|Default|GetVillageMainColor))))
    (:then_3
      ;[1 1 1] WarnItemAvailable
      (CallFunction|WarnItemAvailable))
    (:then_4
      ;[1 1 1] LookForGatherableRessource
      (while (not (Variables|Default|GetStopResearchForRessource))
        (bind _outhit (Collision|SphereTraceForObjects _returnvalue_3 _returnvalue_3 5e+03 (Utilities|Array|MakeArray "ObjectTypeQuery8") false (Variables|Default|GetRessourcePaked) "None"))
        (if (.bblockinghit _outhit)
          (bind _aspack_of_gatherable_ressources (Utilities|Casting|CastToPackOfGatherableRessources (.hitactor _outhit))
            (:then
              (Utilities|Array|Add (Variables|Default|GetRessourcePaked) _aspack_of_gatherable_ressources))
            (:CastFailed
              (Variables|Default|SetStopResearchForRessource true :!label _label)))
          (else
            (goto _label)))))))

(event Collision|EventActorBeginOverlap
  (params (OtherActor :type Actor%20Object%20Reference))
  (|CallParentFunction OtherActor) ; This node is disabled and will not be called.\nDrag off pins to build functionality.
)

(event EventTick
  (params (DeltaSeconds :type Float%20%28single-precision%29))
  (bind _townindicator (Variables|Default|GetTownIndicator))
  (|CallParentFunction DeltaSeconds)
  ;[1 1 1] UpdatePositionIndicator
  (CallFunction|SetWidgetPositionScale _townindicator)
  (CallFunction|SetWidgetRotation _townindicator)
  (CallFunction|SetWidgetOpacity (Variables|/Game/LowPolyProject/Environment/Hud/Town/TownIndicator.TownIndicator_C|GetContainer (Variables|Default|GetTownIndicatorRef))))

(fn ConstructionScript
  (|CallParentFunction))

(fn FindValidBuildingPosition
  (params (BuildingRef :type Building%20BP%20Class%20Reference))
  (bind _buildingwidth (Utilities|GetClassDefaults BuildingRef))
  (for (_array_element _array_index) (Variables|Default|GetValidPointsForCreate)
    (LocalVariables|SetPossibleLocation_Local _array_element)
    (LocalVariables|SetIndexLocal _array_index)
    (bind _returnvalue (Collision|SphereTraceForObjects (LocalVariables|GetPossibleLocation_Local) (LocalVariables|GetPossibleLocation_Local) _buildingwidth (Utilities|Array|MakeArray "ObjectTypeQuery7") false 0 "None"))
    (if (not (or _returnvalue (< (Math|Vector|VectorLength (- (Transformation|GetWorldLocation (Variables|Default|GetStaticMeshComponent)) (LocalVariables|GetPossibleLocation_Local))) (+ _buildingwidth (Variables|Default|GetBuildingWidth)))))
      (Utilities|Array|RemoveIndex (Variables|Default|GetValidPointsForCreate) (LocalVariables|GetIndexLocal))
      (CallFunction|CleanNatureAroundPosition (LocalVariables|GetPossibleLocation_Local) (.BuildingWidth (Utilities|GetClassDefaults BuildingRef)))
      (return true BuildingRef (LocalVariables|GetPossibleLocation_Local) (Math|Rotator|MakeRotator 0.0 0.0 (.yaw (Math|Rotator|MakeRotfromX (- (Transformation|GetWorldLocation (Variables|Default|GetStaticMeshComponent)) (LocalVariables|GetPossibleLocation_Local))))))))
  (return false 0 "0, 0, 0" "0, 0, 0"))

(fn GenerateBuildings
  (bind _habitationlist (Variables|Default|GetHabitationList))
  (bind _buildinglist (Variables|Default|GetBuildingList))
  (Utilities|FlowControl|Sequence
    (:then_0
      ;[1 1 1] Generate valid positions
      (CallFunction|GeneratePositionOfConstruction)
      (Utilities|Array|Shuffle (Variables|Default|GetValidPointsForCreate)))
    (:then_1
      ;[1 1 1] StoreHouse
      (Utilities|FindandConstruct "/Game/LowPolyProject/Environment/Actors/Building/StoreHouse/StoreHouse1/StoreHouse1BP.StoreHouse1BP_C"))
    (:then_2
      ;[1 1 1] Granary
      (Utilities|FindandConstruct "/Game/LowPolyProject/Environment/Actors/Building/StoreHouse/Granary/Granary1/Granary1BP.Granary1BP_C"))
    (:then_3
      ;[1 1 1] HouseBuildings
      (Utilities|FlowControl|ForLoopwithBreak 0 (- (Variables|Default|GetMinHabitation) 1)
        (:LoopBody
          (Utilities|FindandConstruct (Utilities|Array|Get(acopy) _habitationlist (Math|Random|RandomInteger (Utilities|Array|Length _habitationlist))))
          (Variables|Default|SetMaxBuilding (- (Variables|Default|GetMaxBuilding) 1)))
        (:Completed
          ;[1 1 1] OtherBuildings
          (Utilities|FlowControl|ForLoopwithBreak 0 (- (Variables|Default|GetMaxBuilding) 1)
            (:LoopBody
              (Utilities|FindandConstruct (Utilities|Array|Get(acopy) _buildinglist (Math|Random|RandomInteger (Utilities|Array|Length _buildinglist)))))))))))

(fn WarnItemAvailable
  (if (Variables|Default|GetItemAvailable)
    (for _array_element (Variables|Default|GetHabitants)
      (if (Utilities|Name|Equal(Name) (Class|BlackboardComponent|GetValueasName (AI|GetBlackboard (AI|GetAIController _array_element)) (Utilities|Name|MakeLiteralName "Job")) "None")
        (AI|Components|Blackboard|SetValueasBool (AI|GetBlackboard (AI|GetAIController _array_element)) (Utilities|Name|MakeLiteralName "ItemsAvailable") true)))))

(fn WarnUnhabitualBuildingAvailable
  (params (BuildingToWarn :type Building%20BP%20Object%20Reference))
  (for _array_element (Variables|Default|GetHabitants)
    (if (not (.ReturnValue (Utilities|Map|Find (Variables|/Game/LowPolyProject/Environment/Actors/Characters/CharacterBP.CharacterBP_C|GetAlreadyMetBuilding _array_element) BuildingToWarn)))
      (LocalVariables|SetHabitant _array_element)
      (Utilities|Array|Add (Variables|/Game/LowPolyProject/Environment/Actors/Characters/CharacterBP.CharacterBP_C|GetUnhabitualBuildingToSee (LocalVariables|GetHabitant)) BuildingToWarn)
      (AI|Components|Blackboard|SetValueasBool (AI|GetBlackboard (LocalVariables|GetHabitant)) (Utilities|Name|MakeLiteralName "UnhabitualBuilding") true)
      (Default|SetPriority (LocalVariables|GetHabitant) 3 false))))

(fn GeneratePositionOfConstruction
  (bind _townsize (Variables|Default|GetTownSize))
  (bind _townsize_2 (Variables|Default|GetTownSize))
  (for _index (range 0 (- (Variables|Default|GetRayNumber) 1))
    (LocalVariables|SetXVar _index)
    (for _index_2 (range 0 (- (Variables|Default|GetRayNumber) 1))
      (LocalVariables|SetYVar _index_2)
      (bind _outhit (Collision|LineTraceForObjects (+ (+ (Transformation|GetWorldLocation (Variables|Default|GetStaticMeshComponent)) (Math|Vector|MakeVector (Math|Float|MapRangeClamped (Math|Conversions|ToFloat(Integer) (LocalVariables|GetXVar)) 0.0 (Math|Conversions|ToFloat(Integer) (- (Variables|Default|GetRayNumber) 1)) (* _townsize -1.0) _townsize) (Math|Float|MapRangeClamped (Math|Conversions|ToFloat(Integer) (LocalVariables|GetYVar)) 0.0 (Math|Conversions|ToFloat(Integer) (- (Variables|Default|GetRayNumber) 1)) (* _townsize_2 -1.0) _townsize_2) 0.0)) "0, 0,2000.000000") (+ (+ (Transformation|GetWorldLocation (Variables|Default|GetStaticMeshComponent)) (Math|Vector|MakeVector (Math|Float|MapRangeClamped (Math|Conversions|ToFloat(Integer) (LocalVariables|GetXVar)) 0.0 (Math|Conversions|ToFloat(Integer) (- (Variables|Default|GetRayNumber) 1)) (* _townsize -1.0) _townsize) (Math|Float|MapRangeClamped (Math|Conversions|ToFloat(Integer) (LocalVariables|GetYVar)) 0.0 (Math|Conversions|ToFloat(Integer) (- (Variables|Default|GetRayNumber) 1)) (* _townsize_2 -1.0) _townsize_2) 0.0)) "0, 0,-2000.000000") (Utilities|Array|MakeArray "ObjectTypeQuery1") true 0 "None" false))
      (if (and (.bblockinghit _outhit) (> (.Z (Math|Vector|BreakVector (.normal _outhit))) 0.8))
        (Utilities|Array|Add (Variables|Default|GetValidPointsForCreate) (.location _outhit))))))

(fn CleanNatureAroundPosition
  (params (Center :type Vector) (RadiusOfCenter :type Float%20%28single-precision%29))
  (bind _outhit (Collision|SphereTraceForObjects Center Center RadiusOfCenter (Utilities|Array|MakeArray "ObjectTypeQuery8") false 0 "None" :!label _label))
  (while (and (.bblockinghit _outhit) (< (LocalVariables|GetSphereTraceNumber) 100))
    (LocalVariables|SetIndexElement (.hititem _outhit))
    (if (.ReturnValue (Utilities|Map|Find (LocalVariables|GetHitComponents) (.hitcomponent _outhit)))
      (LocalVariables|SetHierarchicalMesh (.Value (Utilities|Map|Find (LocalVariables|GetHitComponents) (.hitcomponent _outhit))))
      (else
        (bind _ashierarchical_instanced_static_mesh_component (Utilities|Casting|CastToHierarchicalInstancedStaticMeshComponent (.hitcomponent _outhit))
          (:then
            (Utilities|Map|Add (LocalVariables|GetHitComponents) (.hitcomponent _outhit) _ashierarchical_instanced_static_mesh_component)
            (LocalVariables|SetHierarchicalMesh _ashierarchical_instanced_static_mesh_component))
          (:CastFailed
            (return)))))
    (Math|Integer|IncrementInt (LocalVariables|GetSphereTraceNumber)
      (:%20%20
        (Class|InstancedStaticMeshComponent|RemoveInstance (LocalVariables|GetHierarchicalMesh) (LocalVariables|GetIndexElement))
        (goto _label)))))