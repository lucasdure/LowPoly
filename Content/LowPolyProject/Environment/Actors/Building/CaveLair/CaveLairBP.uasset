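; Cave lair building actor that spawns random animals at its LairSpawn point, up to MaxAnimalsNumber.
; BeginPlay caches the DebugMode game mode, spawns the first batch and starts a looping 20-second timer to top up the count.
; Each pass picks classes from AnimalsSpawnable, always spawns regardless of collision and records them in AnimalsSpawned.
; Nothing in these graphs removes entries from that array or uses the cached game mode.
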(event EventBeginPlay
  (|CallParentFunction)
  (Utilities|FlowControl|Sequence
    (:then_0
      ;[1 1 1] GameModeRef
      (bind _asdebug_mode (Utilities|Casting|CastToDebugMode (Game|GetGameMode)))
      (Variables|Default|SetGameModeRef _asdebug_mode))
    (:then_1
      ;[1 1 1] SpawnTimer
      (CallFunction|ShouldSpawnAnimals)
      (bind _returnvalue (Utilities|Time|SetTimerbyFunctionName 0 "ShouldSpawnAnimals" 2e+01 true))
      (Variables|Default|SetSpawnTimer _returnvalue))))

(event Collision|EventActorBeginOverlap
  (params (OtherActor :type Actor%20Object%20Reference))
  (|CallParentFunction OtherActor) ; This node is disabled and will not be called.\nDrag off pins to build functionality.
)

(event EventTick
  (params (DeltaSeconds :type Float%20%28single-precision%29))
  (|CallParentFunction DeltaSeconds) ; This node is disabled and will not be called.\nDrag off pins to build functionality.
)

(fn ConstructionScript
  (|CallParentFunction))

(fn ShouldSpawnAnimals
  (bind _animalsspawnable (Variables|Default|GetAnimalsSpawnable))
  (for _index (range 1 (- (Variables|Default|GetMaxAnimalsNumber) (Utilities|Array|Length (Variables|Default|GetAnimalsSpawned))))
    (bind _returnvalue (Game|SpawnActorfromClass (Utilities|Array|Get(acopy) _animalsspawnable (Math|Random|RandomInteger (Utilities|Array|Length _animalsspawnable))) (Math|Transform|MakeTransform (Transformation|GetWorldLocation (Variables|Default|GetLairSpawn)) "0, 0, 0" "1,1,1") "AlwaysSpawn" 0 0))
    (Utilities|Array|Add (Variables|Default|GetAnimalsSpawned) _returnvalue)))