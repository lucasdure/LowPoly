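; PortalBP is a building that teleports an overlapping CharacterBP to the exit of a linked portal.
; On first use without a link, it has the game mode generate a partner portal at Step - 1, activates it and links both ways.
; A state switch drives colors, fluid and collision.
; Portals begin as GuardianToKill, spawning a random guardian pack that holds a back-reference and is cleared on state change.
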(event OnComponentBeginOverlap(PortalDetection)
  (params (OverlappedComponent :type Primitive%20Component%20Object%20Reference) (OtherActor :type Actor%20Object%20Reference) (OtherComp :type Primitive%20Component%20Object%20Reference) (OtherBodyIndex :type Integer) (bFromSweep :type Boolean) (SweepResult :type Hit%20Result%20Structure%20%28by%20ref%29))
  ;[1 1 1] Teleport
  (bind _ascharacter_bp (Utilities|Casting|CastToCharacterBP OtherActor))
  (Variables|Default|SetTeleportedEntity _ascharacter_bp)
  (Utilities|IsValid (Variables|Default|GetLinkedPortal)
    (:Is%20Valid
      _)
    (:Is%20Not%20Valid
      (bind _buildingreturn (Default|GenerateOneBuildinginStep (Variables|/Game/LowPolyProject/GameMode/CameraPawn.CameraPawn_C|GetGameModeRef (Variables|/Game/LowPolyProject/GameMode/StratController.StratController_C|GetPlayerPawnRef (Variables|Default|GetControllerRef))) "PortalBP_C" (- (Variables|Default|GetStep) 1) true true))
      (bind _asportal_bp (Utilities|Casting|CastToPortalBP _buildingreturn))
      (bind _output_get (Variables|Default|SetLinkedPortal _asportal_bp))
      (CallFunction|UpdatePortalState _output_get "NewEnumerator0")
      (Variables|PortalBP_C|SetLinkedPortal _asportal_bp self)))
  (CallFunction|Teleport (Variables|Default|GetLinkedPortal)))

(event EventBeginPlay
  (bind _controllerref (Variables|Default|GetControllerRef))
  (bind _playerpawnref (Variables|/Game/LowPolyProject/GameMode/StratController.StratController_C|GetPlayerPawnRef _controllerref))
  (|CallParentFunction)
  (Utilities|IsValid (Variables|Default|GetControllerRef)
    (:Is%20Valid
      (Utilities|FlowControl|Sequence
        (:then_0
          ;[1 1 1] SetStep
          (Utilities|IsValid _playerpawnref
            (:Is%20Valid
              (Variables|Default|SetStep (Default|GetStepwithCoordinate _playerpawnref (Transformation|GetActorLocation))))))
        (:then_1
          ;[1 1 1] Defaut state
          (CallFunction|UpdatePortalState (Utilities|Select :Index (Math|Random|RandomIntegerinRange 0 1) :Option%200 "NewEnumerator1" :Option%201 "NewEnumerator1")))))))

(event Collision|EventActorBeginOverlap
  (params (OtherActor :type Actor%20Object%20Reference)))

(event EventTick
  (params (DeltaSeconds :type Float%20%28single-precision%29))
  ;[1 1 1] RotateHalo
  (Transformation|AddLocalRotation (Variables|Default|GetPortalHalo) (Math|Rotator|MakeRotator 0.0 0.0 (* (Utilities|Time|GetWorldDeltaSeconds) 2.0)) false false))

(fn ConstructionScript)

(fn Teleport
  (params (PortalToTeleport :type Portal%20BP%20Object%20Reference))
  (Transformation|SetActorLocation (Variables|Default|GetTeleportedEntity) (+ (Math|Vector|MakeVector 0.0 0.0 (Variables|/Script/Engine.CapsuleComponent|GetCapsuleHalfHeight (Variables|/Script/Engine.Character|GetCapsuleComponent (Variables|Default|GetTeleportedEntity)))) (Transformation|GetWorldLocation (Variables|PortalBP_C|GetExit PortalToTeleport))) false false)
  (Components|Movement|StopMovementImmediately (Variables|/Script/Engine.Character|GetCharacterMovement (Variables|Default|GetTeleportedEntity))))

(fn AddGuardians
  (bind _returnvalue (Game|SpawnActorfromClass (Utilities|Array|Get(acopy) (LocalVariables|GetGuardianClass) (Math|Float|Round (* (- (Utilities|Array|Length (LocalVariables|GetGuardianClass)) 1) (Math|Random|RandomFloat)))) (Math|Transform|MakeTransform (Transformation|GetWorldLocation (Variables|Default|GetExit)) (Transformation|GetActorRotation) "1,1,1") "AlwaysSpawn" 0 0))
  (bind _output_get (Variables|Default|SetPackOfGuardian _returnvalue))
  (Variables|/Game/LowPolyProject/Environment/Actors/Characters/PortalGuardians/PacksOfGuardians/PackOfGuardian.PackOfGuardian_C|SetPortal _output_get self))

(fn ActivatePortal
  (Components|Activation|SetActive (Variables|Default|GetPortalFluid) true true)
  (CallFunction|SetParticlesColor "(R=0.104616,G=0.863157,B=0.938686,A=1.000000)")
  (Collision|SetCollisionResponsetoChannel (Variables|Default|GetPortalDetection) "ECC_Pawn" "ECR_Overlap"))

(fn SetParticlesColor
  (params (Param :type Linear%20Color%20Structure))
  (Effects|Components|ParticleSystem|SetColorParameter (Variables|Default|GetPortalGem) "GemColor" Param)
  (Effects|Components|ParticleSystem|SetColorParameter (Variables|Default|GetPortalHalo) "HaloColor" Param))

(fn UpdatePortalState
  (params (Selection :type PortalState%20Enum :default "NewEnumerator0"))
  (CallFunction|ClearPortalState)
  (bind _output_get (Variables|Default|SetState Selection))
  (switch Utilities|FlowControl|Switch|SwitchonPortalState _output_get
    (:NewEnumerator0
      ;[1 1 1] ActivatePortal
      (CallFunction|ActivatePortal))
    (:NewEnumerator2
      ;[1 1 1] GemColor
      (CallFunction|SetParticlesColor "(R=0.166052,G=0.778936,B=0.875000,A=1.000000)"))
    (:NewEnumerator1
      ;[1 1 1] PrepareGuardian
      (CallFunction|SetParticlesColor "(R=0.875000,G=0.496425,B=0.055701,A=1.000000)")
      (CallFunction|AddGuardians))))

(fn ClearPortalState
  (bind _packofguardian (Variables|Default|GetPackOfGuardian))
  (Utilities|IsValid _packofguardian
    (:Is%20Valid
      (Default|ClearGuardians _packofguardian)
      (Actor|DestroyActor _packofguardian))))