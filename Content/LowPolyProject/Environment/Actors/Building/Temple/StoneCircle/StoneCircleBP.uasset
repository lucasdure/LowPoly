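; Temple building actor that forms a ring of instanced rocks, one per player level, which rises when the temple is constructed.
; GenerateStone places randomly yawed instances around a circle, with a fixed-count preview in the construction script.
; On construction it rebuilds the ring, shows a decal and lifts the rocks via the UpRocks timeline, dirtying render state on the final update.
; Aiming toggles custom depth on the rocks.
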(event EventBeginPlay
  (|CallParentFunction))

(event Collision|EventActorBeginOverlap
  (params (OtherActor :type Actor%20Object%20Reference))
  (|CallParentFunction OtherActor) ; This node is disabled and will not be called.\nDrag off pins to build functionality.
)

(event EventTick
  (params (DeltaSeconds :type Float%20%28single-precision%29))
  (|CallParentFunction DeltaSeconds))

(event EventOptionalAim
  (params (Aim :type Boolean))
  ;[1 1 1] Optional mesh to change when aim
  (Rendering|SetRenderCustomDepth (Variables|Default|GetRocks) Aim))

(event EventOnTempleConstruction
  (bind _rocks (Variables|Default|GetRocks))
  (bind _controllerref (Variables|Default|GetControllerRef))
  (bind _returnvalue (Components|InstancedStaticMesh|GetInstanceCount _rocks))
  (bind _playerlevel (Variables|/Game/LowPolyProject/GameMode/StratController.StratController_C|GetPlayerLevel _controllerref))
  (bind _returnvalue_2 (- _returnvalue 1))
  (bind _returnvalue_3 (- _playerlevel 1))
  (bind _returnvalue_4 (Math|Integer|Min(Integer) _returnvalue_3 _returnvalue_2))
  ;[1 1 1] ConstructionEffect
  (Components|InstancedStaticMesh|ClearInstances (Variables|Default|GetRocks))
  (CallFunction|GenerateStone (Variables|/Game/LowPolyProject/GameMode/StratController.StratController_C|GetPlayerLevel (Variables|Default|GetControllerRef)))
  (Rendering|SetVisibility (Variables|Default|GetDecal) true false)
  (bind _height (Timeline|UpRocks PlayFromStart)
    (:Update
      (for _index (range 0 _returnvalue_4)
        (Components|InstancedStaticMesh|UpdateInstanceTransform (Variables|Default|GetRocks) _index (Math|Transform|MakeTransform (Math|Vector|MakeVector (.x (.location (.OutInstanceTransform (Components|InstancedStaticMesh|GetInstanceTransform (Variables|Default|GetRocks) _index false)))) (.y (.location (.OutInstanceTransform (Components|InstancedStaticMesh|GetInstanceTransform (Variables|Default|GetRocks) _index false)))) (Math|Float|MapRangeClamped _height 0.0 1.0 -1.3e+02 0.0)) (.rotation (.OutInstanceTransform (Components|InstancedStaticMesh|GetInstanceTransform (Variables|Default|GetRocks) _index false))) "1,1,1") false (== _index _returnvalue_4) false)))))

(fn ConstructionScript
  (|CallParentFunction)
  (CallFunction|GenerateStone 20))

(fn GenerateStone
  (params (Level :type Integer))
  (for _index (range 0 (- Level 1))
    (Components|InstancedStaticMesh|AddInstance (Variables|Default|GetRocks) (Math|Transform|MakeTransform (Math|Vector|MakeVector (* (Math|Trig|Cos(Radians) (Math|Float|MapRangeClamped (Math|Conversions|ToFloat(Integer) _index) 0.0 (Math|Conversions|ToFloat(Integer) (LocalVariables|GetLastIndex)) 0.0 (* 2 (Math|Trig|GetPI)))) 5e+02) (* (Math|Trig|Sin(Radians) (Math|Float|MapRangeClamped (Math|Conversions|ToFloat(Integer) _index) 0.0 (Math|Conversions|ToFloat(Integer) (LocalVariables|GetLastIndex)) 0.0 (* 2 (Math|Trig|GetPI)))) 5e+02) -1.3e+02) (Math|Rotator|MakeRotator 0.0 0.0 (* (Math|Random|RandomFloat) 3.6e+02)) "1,1,1"))))