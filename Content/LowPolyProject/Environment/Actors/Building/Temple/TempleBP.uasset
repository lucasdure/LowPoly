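; Temple building Blueprint, a child of a parent building class, that registers itself with its town center when constructed.
; OnConstructed runs the parent logic, adds the temple to the town center's Temples array and calls WarnUnhabitualBuildingAvailable on it.
; It then fires OnTempleConstruction, an event left empty here; BeginPlay and the construction script only call the parent.
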(event Custom|OnTempleConstruction)

(event EventBeginPlay
  (|CallParentFunction))

(event Collision|EventActorBeginOverlap
  (params (OtherActor :type Actor%20Object%20Reference))
  (|CallParentFunction OtherActor) ; This node is disabled and will not be called.\nDrag off pins to build functionality.
)

(event EventTick
  (params (DeltaSeconds :type Float%20%28single-precision%29))
  (|CallParentFunction DeltaSeconds) ; This node is disabled and will not be called.\nDrag off pins to build functionality.
)

(event EventOnConstructed
  ;[1 1 1] TempleConstruction
  (|CallParentFunction)
  (Utilities|Array|Add (Variables|/Game/LowPolyProject/Environment/Actors/Building/TownCenters/TownCenterBP.TownCenterBP_C|GetTemples (Variables|Default|GetTownCenterRef)) self)
  (Default|WarnUnhabitualBuildingAvailable (Variables|Default|GetTownCenterRef) self)
  (CallFunction|OnTempleConstruction))

(fn ConstructionScript
  (|CallParentFunction))