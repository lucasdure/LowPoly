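; GiantGateBP is a giant environment gate that opens by sliding a ring of door pieces apart like an iris.
; The construction script spawns twelve static mesh doors at even yaw steps around a full circle and stores them in an array.
; The OpenGate event plays a timeline that moves each door out along its own forward vector from the central static mesh's location, without sweep.
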(event Custom|OpenGate
  ;[1 1 1] OpenGate
  (bind _opening (Timeline|OpenGateTimeLine PlayFromStart)
    (:Update
      (for _array_element (Variables|Default|GetDoors)
        (Transformation|SetWorldLocation _array_element (+ (* (Math|Vector|GetForwardVector _array_element) (* 10000 _opening)) (Transformation|GetWorldLocation (Variables|Default|GetStaticMeshComponent))) false false)))))

(event EventBeginPlay
  (|CallParentFunction))

(event Collision|EventActorBeginOverlap
  (params (OtherActor :type Actor%20Object%20Reference))
  (|CallParentFunction OtherActor) ; This node is disabled and will not be called.\nDrag off pins to build functionality.
)

(event EventTick
  (params (DeltaSeconds :type Float%20%28single-precision%29))
  (|CallParentFunction DeltaSeconds) ; This node is disabled and will not be called.\nDrag off pins to build functionality.
)

(fn ConstructionScript
  (|CallParentFunction)
  (for _index (range 0 11)
    (bind _returnvalue (AddComponent|AddStaticMeshComponent false (Math|Transform|MakeTransform "0, 0, 0" (Math|Rotator|MakeRotator 0.0 0.0 (Math|Conversions|ToFloat(Integer) (* _index 30))) "1,1,1")))
    (Utilities|Array|Add (Variables|Default|GetDoors) _returnvalue)))