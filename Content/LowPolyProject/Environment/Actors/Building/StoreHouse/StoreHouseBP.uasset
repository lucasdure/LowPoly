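; Storage building for a town, also handling the granary variant, that holds resources in a grid of spawned StoreArea actors.
; Once controller and HUD are valid, it registers with the TownCenter, builds the grid and seeds random starting amounts of matching resources.
; TransfertRessource fills or drains areas up to per-resource capacity, updating stock records, visuals and HUD.
; Reservations adjust a separate unreserved count, and new stock can flag item availability to the town.
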(event EventBeginPlay
  (|CallParentFunction))

(event Collision|EventActorBeginOverlap
  (params (OtherActor :type Actor%20Object%20Reference))
  (|CallParentFunction OtherActor) ; This node is disabled and will not be called.\nDrag off pins to build functionality.
)

(event EventTick
  (params (DeltaSeconds :type Float%20%28single-precision%29))
  (|CallParentFunction DeltaSeconds) ; This node is disabled and will not be called.\nDrag off pins to build functionality.
)

(event EventSetTownCenterRef
  (params (TownCenterRef :type Town%20Center%20BP%20Object%20Reference))
  (bind _self self)
  (bind _controllerref (Variables|Default|GetControllerRef))
  ;[1 1 1] Set Town ref + Random ressources
  (Utilities|IsValid _controllerref :!label _label
    (:Is%20Valid
      (Utilities|IsValid (Variables|/Game/LowPolyProject/GameMode/StratController.StratController_C|GetStratHudRef _controllerref)
        (:Is%20Valid
          (bind _output_get (Variables|Default|SetTownCenterRef TownCenterRef))
          (if (Variables|Default|GetGranary)
            (bind _asgranary_bp (Utilities|Casting|CastToGranaryBP _self))
            (Variables|/Game/LowPolyProject/Environment/Actors/Building/TownCenters/TownCenterBP.TownCenterBP_C|SetGranaryRef _output_get _asgranary_bp)
            (else
              (Variables|/Game/LowPolyProject/Environment/Actors/Building/TownCenters/TownCenterBP.TownCenterBP_C|SetStoreHouseRef _output_get _self)))
          (CallFunction|AddStoreAreas)
          (for (_array_element _array_index) (Variables|/Game/LowPolyProject/Environment/Actors/Building/TownCenters/TownCenterBP.TownCenterBP_C|GetMinBrutRessource (Variables|Default|GetTownCenterRef))
            (if (Math|Boolean|Equal(Boolean) (Variables|Default|GetGranary) (Utilities|GetClassDefaults (.ressource _array_element)))
              (CallFunction|TransfertRessource (.ressource _array_element) 0 (Math|Float|Round (Math|Float|MapRangeClamped (Math|Random|RandomFloat) 0.0 1.0 (Math|Conversions|ToFloat(Integer) (.amount _array_element)) (Math|Conversions|ToFloat(Integer) (.amount (Utilities|Array|Get(acopy) (Variables|/Game/LowPolyProject/Environment/Actors/Building/TownCenters/TownCenterBP.TownCenterBP_C|GetMaxBrutRessource (Variables|Default|GetTownCenterRef)) _array_index))))) false))))
        (:Is%20Not%20Valid
          (Utilities|FlowControl|Delay 0.0 :!label _label_2)
          (goto _label))))
    (:Is%20Not%20Valid
      (goto _label_2))))

(fn ConstructionScript
  (|CallParentFunction))

(fn AddStoreAreas
  (bind _xywidth (Variables|Default|GetXYWidth))
  (bind _sizestore (Variables|Default|GetSizeStore))
  (bind _spawnposition (Variables|Default|GetSpawnPosition))
  (bind _xywidth_2 (Variables|Default|GetXYWidth))
  (bind _xywidth_3 (Variables|Default|GetXYWidth))
  (bind _sizestore_2 (Variables|Default|GetSizeStore))
  (bind _xywidth_4 (Variables|Default|GetXYWidth))
  (bind _returnvalue (Transformation|GetWorldRotation _spawnposition))
  (LocalVariables|SetOffset (Math|Vector|RotateVector (select (== (Math|Float|Min(Float) (.x _xywidth_4) (.y _xywidth_4)) (.x _xywidth_4)) (Math|Vector|MakeVector (* (* (Variables|Default|GetSizeStore) (/ (- (.x _xywidth_4) (.y _xywidth_4)) (- (.y _xywidth_4) 1.0))) -1.0) 0.0 0.0) (Math|Vector|MakeVector 0.0 (* (* (Variables|Default|GetSizeStore) (/ (- (.y _xywidth_4) (.x _xywidth_4)) (- (.x _xywidth_4) 1.0))) -1.0) 0.0)) (Transformation|GetWorldRotation (Variables|Default|GetSpawnPosition))))
  (for _index (range 0 (- (Math|Float|Truncate (.x _xywidth_2)) 1))
    (LocalVariables|SetX _index)
    (for _index_2 (range 0 (- (Math|Float|Truncate (.y _xywidth_2)) 1))
      (LocalVariables|SetY _index_2)
      (bind _returnvalue_2 (Game|SpawnActorfromClass "/Game/LowPolyProject/Environment/Actors/Building/StoreHouse/StoreArea.StoreArea_C" (Math|Transform|MakeTransform (+ (Transformation|GetWorldLocation _spawnposition) (Math|Vector|RotateVector (Math|Vector|MakeVector (Math|Float|MapRangeClamped (Math|Conversions|ToFloat(Integer) (LocalVariables|GetX)) 0.0 (- (Math|Float|Max(Float) (.x _xywidth_3) (.y _xywidth_3)) 1.0) (* -1 _sizestore_2) _sizestore_2) (Math|Float|MapRangeClamped (Math|Conversions|ToFloat(Integer) (LocalVariables|GetY)) 0.0 (- (Math|Float|Max(Float) (.x _xywidth) (.y _xywidth)) 1.0) (* -1 _sizestore) _sizestore) 0.0) _returnvalue) (LocalVariables|GetOffset)) _returnvalue "1,1,1") "AlwaysSpawn" 0 0))
      (Utilities|Array|Add (Variables|Default|GetStoreAreas) _returnvalue_2))))

(fn StoreOneRessource
  (params (RessourceToAdd :type Brut%20Ressource%20BP%20Class%20Reference) (Amount :type Integer))
  (bind _output_get (LocalVariables|SetRessourceToAddLocal RessourceToAdd))
  (LocalVariables|SetAmountLocal Amount)
  (LocalVariables|SetMaxAmount (Math|Float|Round (* (.x (.RessourceXYZWidthInStore (Utilities|GetClassDefaults _output_get))) (.y (.RessourceXYZWidthInStore (Utilities|GetClassDefaults _output_get))) (.z (.RessourceXYZWidthInStore (Utilities|GetClassDefaults _output_get))))))
  (bind _index (Utilities|FlowControl|ForLoopwithBreak (Variables|Default|GetStoreAreaIndex) (- (Utilities|Array|Length (Variables|Default|GetStoreAreas)) 1) :!label _label)
    (:LoopBody
      (Variables|/Game/LowPolyProject/Environment/Actors/Building/StoreHouse/StoreArea.StoreArea_C|SetRessource (Utilities|Array|Get(acopy) (Variables|Default|GetStoreAreas) _index) (Utilities|Struct|MakeRessourceAmount (LocalVariables|GetRessourceToAddLocal) (select (> (LocalVariables|GetAmountLocal) (LocalVariables|GetMaxAmount)) (LocalVariables|GetMaxAmount) (LocalVariables|GetAmountLocal)) (Utilities|Array|MakeArray 0) (select (> (LocalVariables|GetAmountLocal) (LocalVariables|GetMaxAmount)) (LocalVariables|GetMaxAmount) (LocalVariables|GetAmountLocal))))
      (LocalVariables|SetAmountLocal (- (LocalVariables|GetAmountLocal) (select (> (LocalVariables|GetAmountLocal) (LocalVariables|GetMaxAmount)) (LocalVariables|GetMaxAmount) (LocalVariables|GetAmountLocal))))
      (Default|SetVisualRessource (Utilities|Array|Get(acopy) (Variables|Default|GetStoreAreas) _index))
      (Utilities|Array|Add (LocalVariables|GetStoresAreasLocal) (Utilities|Array|Get(acopy) (Variables|Default|GetStoreAreas) _index))
      (if (== (LocalVariables|GetAmountLocal) 0)
        (Variables|Default|SetStoreAreaIndex (+ _index 1))
        (goto _label Break)))
    (:Completed
      (Utilities|Array|Add (Variables|Default|GetStoredRessource) (Utilities|Struct|MakeRessourceAmount (LocalVariables|GetRessourceToAddLocal) Amount (LocalVariables|GetStoresAreasLocal) Amount))
      (if (.IsItem (Utilities|GetClassDefaults (LocalVariables|GetRessourceToAddLocal)))
        _))))

(fn TransfertRessource
  (params (RessourceClass :type Brut%20Ressource%20BP%20Class%20Reference) (CharacterRef :type Character%20BP%20Object%20Reference) (Amount :type Integer) (TakeFromStore :type Boolean))
  (bind _controllerref (Variables|Default|GetControllerRef))
  (bind _controllerref_2 (Variables|Default|GetControllerRef))
  (bind _controllerref_3 (Variables|Default|GetControllerRef))
  (bind _controllerref_4 (Variables|Default|GetControllerRef))
  (bind _ressourcexyzwidthinstore (Utilities|GetClassDefaults RessourceClass))
  (bind _strathudref (Variables|/Game/LowPolyProject/GameMode/StratController.StratController_C|GetStratHudRef _controllerref_2))
  (bind _strathudref_2 (Variables|/Game/LowPolyProject/GameMode/StratController.StratController_C|GetStratHudRef _controllerref_3))
  (bind _strathudref_3 (Variables|/Game/LowPolyProject/GameMode/StratController.StratController_C|GetStratHudRef _controllerref))
  (bind _strathudref_4 (Variables|/Game/LowPolyProject/GameMode/StratController.StratController_C|GetStratHudRef _controllerref_4))
  (if TakeFromStore
    (bind (_array_element _array_index) (Utilities|Array|ForEachLoopwithBreak (Variables|Default|GetStoredRessource) :!label _label)
      (:LoopBody
        (if (== (.ressource _array_element) RessourceClass)
          (LocalVariables|SetRessourceIndex _array_index)
          (Utilities|FlowControl|Sequence
            (:then_0
              (bind _arrayelement (Utilities|Array|ReverseforEachLoop (.storearearef (Utilities|Array|Get(acopy) (Variables|Default|GetStoredRessource) _array_index)))
                (:LoopBody
                  (if (not (== (LocalVariables|GetAmountTakenSuccesfully) Amount))
                    (LocalVariables|SetRessourceTakenInThisStoreArea (select (> (- Amount (LocalVariables|GetAmountTakenSuccesfully)) (.amount (Variables|/Game/LowPolyProject/Environment/Actors/Building/StoreHouse/StoreArea.StoreArea_C|GetRessource _arrayelement))) (.amount (Variables|/Game/LowPolyProject/Environment/Actors/Building/StoreHouse/StoreArea.StoreArea_C|GetRessource _arrayelement)) (- Amount (LocalVariables|GetAmountTakenSuccesfully))))
                    (Utilities|Struct|SetmembersinRessourceAmount (Utilities|Array|Get(acopy) (Variables|Default|GetStoredRessource) (LocalVariables|GetRessourceIndex)) (- (Utilities|Struct|BreakRessourceAmount (Utilities|Array|Get(acopy) (Variables|Default|GetStoredRessource) (LocalVariables|GetRessourceIndex))) (LocalVariables|GetRessourceTakenInThisStoreArea)))
                    (Utilities|Struct|SetmembersinRessourceAmount (Variables|/Game/LowPolyProject/Environment/Actors/Building/StoreHouse/StoreArea.StoreArea_C|GetRessource _arrayelement) (select (== (- (.amount (Variables|/Game/LowPolyProject/Environment/Actors/Building/StoreHouse/StoreArea.StoreArea_C|GetRessource _arrayelement)) (LocalVariables|GetRessourceTakenInThisStoreArea)) 0) 0 (Utilities|Struct|BreakRessourceAmount (Variables|/Game/LowPolyProject/Environment/Actors/Building/StoreHouse/StoreArea.StoreArea_C|GetRessource _arrayelement))) (- (.amount (Variables|/Game/LowPolyProject/Environment/Actors/Building/StoreHouse/StoreArea.StoreArea_C|GetRessource _arrayelement)) (LocalVariables|GetRessourceTakenInThisStoreArea)))
                    (LocalVariables|SetAmountTakenSuccesfully (+ (LocalVariables|GetAmountTakenSuccesfully) (LocalVariables|GetRessourceTakenInThisStoreArea)))))))
            (:then_1
              (goto _label Break)))))
      (:Completed
        (bind _arrayelement_2 (Utilities|Array|ReverseforEachLoop (.storearearef (Utilities|Array|Get(acopy) (Variables|Default|GetStoredRessource) (LocalVariables|GetRessourceIndex))))
          (:LoopBody
            (Default|SetVisualRessource _arrayelement_2)
            (if (<= (.amount (Variables|/Game/LowPolyProject/Environment/Actors/Building/StoreHouse/StoreArea.StoreArea_C|GetRessource _arrayelement_2)) 0)
              (Utilities|Array|Clear (.storearearef (Utilities|Array|Get(acopy) (Variables|Default|GetStoredRessource) (LocalVariables|GetRessourceIndex))))))
          (:Completed
            (Default|RightHandIcone _strathudref_3 CharacterRef)
            (Default|LeftHandIcone _strathudref_3 CharacterRef)
            (if (== (Variables|Default|GetTownCenterRef) (Variables|/Game/LowPolyProject/Environment/Hud/Camera/StrategicHud.StrategicHud_C|GetTownSelected (Variables|/Game/LowPolyProject/GameMode/StratController.StratController_C|GetStratHudRef (Variables|Default|GetControllerRef))))
              (Default|UpdateRessourceVisual _strathudref))
            (Default|UpdateItemInventory _strathudref self)
            (return (LocalVariables|GetAmountTakenSuccesfully))))))
    (else
      (LocalVariables|SetAmountToGive Amount)
      (LocalVariables|SetMaxAmount (Math|Float|Round (* (.x _ressourcexyzwidthinstore) (.y _ressourcexyzwidthinstore) (.z _ressourcexyzwidthinstore))))
      (bind (_array_element_2 _array_index_2) (Utilities|Array|ForEachLoopwithBreak (Variables|Default|GetStoredRessource) :!label _label_2)
        (:LoopBody
          (if (== (.ressource _array_element_2) RessourceClass)
            (LocalVariables|SetRessourceIndex _array_index_2)
            (bind (_amounttogiveresult _storesareasresult) (CallFunction|StoreinStoreArea (.storearearef _array_element_2) RessourceClass (LocalVariables|GetAmountToGive) (LocalVariables|GetMaxAmount)))
            (LocalVariables|SetStoreAreasAlreafyFilled _storesareasresult)
            (LocalVariables|SetAmountToGive _amounttogiveresult)
            (goto _label_2 Break)))
        (:Completed
          (bind (_amounttogiveresult_2 _storesareasresult_2) (CallFunction|StoreinStoreArea (Variables|Default|GetStoreAreas) RessourceClass (LocalVariables|GetAmountToGive) (LocalVariables|GetMaxAmount)))
          (bind _output_get (LocalVariables|SetStoresAreasLocal _storesareasresult_2))
          (for _array_element_3 (LocalVariables|GetStoreAreasAlreafyFilled)
            (Utilities|Array|RemoveItem _output_get _array_element_3))
          (Utilities|Array|AppendArray _output_get (LocalVariables|GetStoreAreasAlreafyFilled))
          (LocalVariables|SetAmountToGive _amounttogiveresult_2)
          (if (and (> (- Amount (LocalVariables|GetAmountToGive)) 0) (Utilities|GetClassDefaults RessourceClass))
            (Variables|/Game/LowPolyProject/Environment/Actors/Building/TownCenters/TownCenterBP.TownCenterBP_C|SetItemAvailable (Variables|Default|GetTownCenterRef) true)
            (Default|WarnItemAvailable (Variables|Default|GetTownCenterRef)))
          (if (== (LocalVariables|GetRessourceIndex) -1)
            (Utilities|Array|Add (Variables|Default|GetStoredRessource) (Utilities|Struct|MakeRessourceAmount RessourceClass (- Amount (LocalVariables|GetAmountToGive)) (LocalVariables|GetStoresAreasLocal) (- Amount (LocalVariables|GetAmountToGive))))
            (else
              (Utilities|Struct|SetmembersinRessourceAmount (Utilities|Array|Get(acopy) (Variables|Default|GetStoredRessource) (LocalVariables|GetRessourceIndex)) (+ (.Amount (Utilities|Struct|BreakRessourceAmount (Utilities|Array|Get(acopy) (Variables|Default|GetStoredRessource) (LocalVariables|GetRessourceIndex)))) (- Amount (LocalVariables|GetAmountToGive))) (LocalVariables|GetStoresAreasLocal) (+ (.AmountNoReserved (Utilities|Struct|BreakRessourceAmount (Utilities|Array|Get(acopy) (Variables|Default|GetStoredRessource) (LocalVariables|GetRessourceIndex)))) (- Amount (LocalVariables|GetAmountToGive))))))
          (Utilities|IsValid CharacterRef
            (:Is%20Valid
              (Default|RightHandIcone _strathudref_4 CharacterRef)
              (Default|LeftHandIcone _strathudref_4 CharacterRef))
            (:Is%20Not%20Valid
              _))
          (if (== (Variables|Default|GetTownCenterRef) (Variables|/Game/LowPolyProject/Environment/Hud/Camera/StrategicHud.StrategicHud_C|GetTownSelected (Variables|/Game/LowPolyProject/GameMode/StratController.StratController_C|GetStratHudRef (Variables|Default|GetControllerRef))))
            (Default|UpdateRessourceVisual _strathudref_2))
          (Default|UpdateItemInventory _strathudref_2 self)
          (return (- Amount (LocalVariables|GetAmountToGive))))))))

(fn FreeorReserveRessource
  (params (RessourceToFree :type Brut%20Ressource%20BP%20Class%20Reference) (AmountToFree :type Integer) (Reserve :type Boolean))
  (bind _storedressource (Variables|Default|GetStoredRessource))
  (bind (_array_element _array_index) (Utilities|Array|ForEachLoopwithBreak _storedressource)
    (:LoopBody
      (if (== (.ressource _array_element) RessourceToFree)
        (bind _structout (Utilities|Struct|SetmembersinRessourceAmount (Utilities|Array|Get(acopy) _storedressource _array_index) (+ (Utilities|Struct|BreakRessourceAmount (Utilities|Array|Get(acopy) _storedressource _array_index)) (* AmountToFree (select Reserve -1 1)))))
        (if (Utilities|GetClassDefaults (.ressource _structout))
          (Variables|/Game/LowPolyProject/Environment/Actors/Building/TownCenters/TownCenterBP.TownCenterBP_C|SetItemAvailable (Variables|Default|GetTownCenterRef) true))
        (return)))
    (:Completed
      (return))))

(fn StoreinStoreArea
  (params (StoreAreas :type Array%20of%20Store%20Area%20Object%20References) (RessourceClass :type Brut%20Ressource%20BP%20Class%20Reference) (AmountToGive :type Integer) (MaxAmount :type Integer))
  (LocalVariables|SetRessourceClassLocal RessourceClass)
  (LocalVariables|SetAmountToGiveLocal AmountToGive)
  (LocalVariables|SetMaxAmountLocal MaxAmount)
  (bind _array_element (Utilities|Array|ForEachLoopwithBreak StoreAreas :!label _label)
    (:LoopBody
      (if (or (== (.ressource (Variables|/Game/LowPolyProject/Environment/Actors/Building/StoreHouse/StoreArea.StoreArea_C|GetRessource _array_element)) 0) (== (.ressource (Variables|/Game/LowPolyProject/Environment/Actors/Building/StoreHouse/StoreArea.StoreArea_C|GetRessource _array_element)) (LocalVariables|GetRessourceClassLocal)))
        (bind _output_get (LocalVariables|SetAmountGivenThisTurn (select (> (LocalVariables|GetAmountToGiveLocal) (- (LocalVariables|GetMaxAmountLocal) (.amount (Variables|/Game/LowPolyProject/Environment/Actors/Building/StoreHouse/StoreArea.StoreArea_C|GetRessource _array_element)))) (- (LocalVariables|GetMaxAmountLocal) (.amount (Variables|/Game/LowPolyProject/Environment/Actors/Building/StoreHouse/StoreArea.StoreArea_C|GetRessource _array_element))) (LocalVariables|GetAmountToGiveLocal))))
        (Variables|/Game/LowPolyProject/Environment/Actors/Building/StoreHouse/StoreArea.StoreArea_C|SetRessource _array_element (Utilities|Struct|MakeRessourceAmount (LocalVariables|GetRessourceClassLocal) (+ (.amount (Variables|/Game/LowPolyProject/Environment/Actors/Building/StoreHouse/StoreArea.StoreArea_C|GetRessource _array_element)) _output_get) (Utilities|Array|MakeArray) (+ (.amount (Variables|/Game/LowPolyProject/Environment/Actors/Building/StoreHouse/StoreArea.StoreArea_C|GetRessource _array_element)) _output_get)))
        (LocalVariables|SetAmountToGiveLocal (- (LocalVariables|GetAmountToGiveLocal) (LocalVariables|GetAmountGivenThisTurn)))
        (Default|SetVisualRessource _array_element)
        (Utilities|Array|Add (LocalVariables|GetStoresAreasLocal) _array_element)
        (if (== (LocalVariables|GetAmountToGiveLocal) 0)
          (goto _label Break))))
    (:Completed
      (return (LocalVariables|GetAmountToGiveLocal) (LocalVariables|GetStoresAreasLocal)))))