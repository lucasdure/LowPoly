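; Buildable switch-operated elevator whose physics-simulated platform hangs from a cable and moves up or down.
; A timeline spins the cable and grows or shrinks a constraint's linear limit, stopping at zero or on box overlap.
; On construction or non-ghost start, it spawns a linked ground switch alongside the child-actor one.
; Placement checks box-trace eight surrounding points for open space, snapping and rotating the elevator against the edge.
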(event OnComponentBeginOverlap(Box)
  (params (OverlappedComponent :type Primitive%20Component%20Object%20Reference) (OtherActor :type Actor%20Object%20Reference) (OtherComp :type Primitive%20Component%20Object%20Reference) (OtherBodyIndex :type Integer) (bFromSweep :type Boolean) (SweepResult :type Hit%20Result%20Structure%20%28by%20ref%29))
  ;[1 1 1] Make Elevator Go Up Or Down
  (CallFunction|StopElevator))

(event Custom|StopElevator
  ;[1 1 1] Make Elevator Go Up Or Down
  (bind _rotationvalue (Timeline|MoveCable Stop)
    (:Update
      (Transformation|SetRelativeRotation (Variables|Default|GetCable) (Math|Rotator|MakeRotator 0.0 (* 360 _rotationvalue) 0.0) false false)
      (bind _output_get (Variables|Default|SetLinearLimit (Math|Float|Clamp(Float) (+ (* (Utilities|Time|GetWorldDeltaSeconds) (select (Variables|Default|GetGoDown) 6e+01 -6e+01)) (Variables|Default|GetLinearLimit)) 0.0 1e+06)))
      (Class|PhysicsConstraintComponent|SetLinearXLimit (Variables|Default|GetCableStrengh) "LCM_Limited" _output_get)
      (if (== (Variables|Default|GetLinearLimit) 0.0)
        (CallFunction|StopElevator)))))

(event EventBeginPlay
  ;[1 1 1] Put switch
  (|CallParentFunction)
  (Utilities|FlowControl|Delay 1.0)
  (if (not (Variables|Default|GetIsGhost))
    (CallFunction|SpawnSwitch)))

(event Collision|EventActorBeginOverlap
  (params (OtherActor :type Actor%20Object%20Reference))
  (|CallParentFunction OtherActor) ; This node is disabled and will not be called.\nDrag off pins to build functionality.
)

(event EventTick
  (params (DeltaSeconds :type Float%20%28single-precision%29))
  (|CallParentFunction DeltaSeconds))

(event EventActivateActors
  (params (Activate :type Boolean) (ActivationType :type Integer))
  ;[1 1 1] Make Elevator Go Up Or Down
  (bind _output_get (Variables|Default|SetGoDown Activate))
  (Class|PrimitiveComponent|WakeRigidBody (Variables|Default|GetElevatorMesh) "None")
  (if _output_get
    (bind _rotationvalue (Timeline|MoveCable Play)
      (:Update
        (Transformation|SetRelativeRotation (Variables|Default|GetCable) (Math|Rotator|MakeRotator 0.0 (* 360 _rotationvalue) 0.0) false false)
        (bind _output_get_2 (Variables|Default|SetLinearLimit (Math|Float|Clamp(Float) (+ (* (Utilities|Time|GetWorldDeltaSeconds) (select (Variables|Default|GetGoDown) 6e+01 -6e+01)) (Variables|Default|GetLinearLimit)) 0.0 1e+06)))
        (Class|PhysicsConstraintComponent|SetLinearXLimit (Variables|Default|GetCableStrengh) "LCM_Limited" _output_get_2)
        (if (== (Variables|Default|GetLinearLimit) 0.0)
          (CallFunction|StopElevator))))
    (else
      (Timeline|MoveCable Reverse))))

(event EventOptionalAim
  (params (Aim :type Boolean))
  ;[1 1 1] Aim optional
  (Rendering|SetCustomDepthStencilValue (Variables|Default|GetElevatorMesh) (Variables|Default|GetRelation))
  (Rendering|SetRenderCustomDepth (Variables|Default|GetElevatorMesh) Aim))

(event EventOnConstructed
  ;[1 1 1] Put switch
  (|CallParentFunction)
  (CallFunction|SpawnSwitch))

(fn ConstructionScript
  (|CallParentFunction)
  (Utilities|FlowControl|Sequence
    (:then_0
      ;[1 1 1] Add elevator link
      (bind _asswitch_bp (Utilities|Casting|CastToSwitchBP (Variables|/Script/Engine.ChildActorComponent|GetChildActor (Variables|Default|GetChildActor))))
      (bind _output_get (Variables|Default|SetAdditionalSwitch _asswitch_bp))
      (Utilities|Array|Add (Variables|/Game/LowPolyProject/Environment/Actors/Furniture/ActivatorBP.ActivatorBP_C|GetActorToActivate _output_get) (Utilities|Struct|MakeActivationControl self 0)))))

(fn AdditionnalBuildingConstructionNeeds
  (bind _returnvalue (Transformation|GetActorLocation))
  (bind _returnvalue_2 (- _returnvalue "0, 0,2.000000"))
  (|CallParentFunction)
  (for _index (range 0 7)
    (bind _output_get (LocalVariables|SetIndexLocal _index))
    (bind (_circleposition _contact) (CallFunction|TraceLineAroundBuilding _output_get))
    (if (not _contact)
      (Transformation|SetActorRotation (Math|Rotator|MakeRotator 0.0 0.0 (.yaw (Math|Rotator|FindLookatRotation (Transformation|GetWorldLocation (Variables|Default|GetStaticMeshComponent)) _circleposition))))
      (bind _circleposition_2 (Class|SimpleMathFunction|GetCirclePoint (LocalVariables|GetIndexLocal) 8 397.0 _returnvalue_2))
      (bind _outhit (Collision|LineTraceForObjects _circleposition_2 _returnvalue_2 (Utilities|Array|MakeArray "ObjectTypeQuery1") false 0 "None"))
      (Transformation|SetActorLocation (+ (.Location (Collision|BreakHitResult _outhit)) (Math|Vector|RotateVector "206.000000, 0, 0" (Math|Rotator|FindLookatRotation _circleposition_2 _returnvalue_2))) false false)
      (bind _contact_2 (CallFunction|TraceLineAroundBuilding (LocalVariables|GetIndexLocal)))
      (if (not _contact_2)
        (bind _circleposition_3 (Class|SimpleMathFunction|GetCirclePoint (LocalVariables|GetIndexLocal) 8 205.0 (Transformation|GetActorLocation)))
        (bind _returnvalue_3 (Collision|LineTraceForObjects (+ _circleposition_3 "0, 0,400.000000") (+ _circleposition_3 "0, 0,-400.000000") (Utilities|Array|MakeArray "ObjectTypeQuery1") false 0 "None"))
        (if _returnvalue_3
          (return true)))))
  (return false))

(fn SpawnSwitch
  (bind _staticmeshcomponent (Variables|Default|GetStaticMeshComponent))
  (bind _returnvalue (Transformation|GetWorldRotation _staticmeshcomponent))
  (bind _returnvalue_2 (Transformation|GetWorldLocation _staticmeshcomponent))
  (Rendering|SetVisibility (Variables|Default|GetChildActor) true false)
  (Class|PhysicsConstraintComponent|SetConstrainedComponents (Variables|Default|GetCableStrengh) (Variables|Default|GetAttachLink) "None" (Variables|Default|GetElevatorMesh) "None")
  (Physics|SetSimulatePhysics (Variables|Default|GetElevatorMesh) true)
  (bind (_outhit _returnvalue_3) (Collision|LineTraceForObjects (+ (Math|Vector|RotateVector "0,200.000000,400.000000" _returnvalue) _returnvalue_2) (+ _returnvalue_2 (Math|Vector|RotateVector "0,200.000000,-400.000000" _returnvalue)) (Utilities|Array|MakeArray "ObjectTypeQuery1") false 0 "ForOneFrame" true "(R=1.000000,G=0.000000,B=0.000000,A=1.000000)" "(R=0.000000,G=1.000000,B=0.000000,A=1.000000)" 1e+01))
  (if _returnvalue_3
    (bind _returnvalue_4 (Game|SpawnActorfromClass "/Game/LowPolyProject/Environment/Actors/Furniture/Switch/SwitchBP.SwitchBP_C" (Math|Transform|MakeTransform (.Location (Collision|BreakHitResult _outhit)) (Transformation|GetWorldRotation (Variables|Default|GetStaticMeshComponent)) "1,1,1") "AlwaysSpawn" 0 0))
    (Utilities|Array|Add (Variables|/Game/LowPolyProject/Environment/Actors/Furniture/ActivatorBP.ActivatorBP_C|GetActorToActivate _returnvalue_4) (Utilities|Struct|MakeActivationControl self 0))))

(fn TraceLineAroundBuilding
  (params (Index :type Integer))
  (bind _circleposition (Class|SimpleMathFunction|GetCirclePoint Index 8 397.0 (Transformation|GetActorLocation)))
  (bind _returnvalue (Class|KismetSystemLibrary|BoxTraceMultiforObjects (+ _circleposition "0, 0,400.000000") (+ _circleposition "0, 0,-400.000000") "167.000000,167.000000,0.000000" "0, 0, 0" (Utilities|Array|MakeArray "ObjectTypeQuery1") false 0 "None" true))
  (return _circleposition _returnvalue))