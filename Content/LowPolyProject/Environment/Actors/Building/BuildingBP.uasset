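; Base building actor for the strategy game, covering placement ghost, resource-fed construction and the finished, selectable structure.
; BeginPlay registers it on the map, flattens terrain and links its stat bar; selection drives outline, HUD, light and roof hiding.
; Ghosts track the nearest TownCenter in range, which records completed buildings.
; Construction tracks delivered and per-character reserved resources to cap progress, shown through dynamic material parameters.
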(event Custom|SetTownCenterRef
  (params (TownCenterRef :type Town%20Center%20BP%20Object%20Reference)))

(event Custom|OnConstructed
  ;[1 1 1] OnConstructed
  (CallFunction|SetBuildAdvancement 1.0)
  (CallFunction|SetGhostMode "QueryAndPhysics")
  (Utilities|Array|Add (Variables|/Game/LowPolyProject/Environment/Actors/Building/TownCenters/TownCenterBP.TownCenterBP_C|GetBuildingBuilded (Variables|Default|GetTownCenterRef)) self)
  (Utilities|Array|RemoveItem (Variables|/Game/LowPolyProject/Environment/Actors/Building/TownCenters/TownCenterBP.TownCenterBP_C|GetBuildingWaitingBuilder (Variables|Default|GetTownCenterRef)) self)
  (Variables|Default|SetLifePoint (Variables|Default|GetMaxLifePoint))
  (Default|SetLifeBarFunction (Variables|Default|GetBarStatRef))
  (if (CallFunction|ShoudUpdateProperties)
    (Default|UpdatePropertiesOfTable (Variables|/Game/LowPolyProject/GameMode/StratController.StratController_C|GetStratHudRef (Variables|Default|GetControllerRef)) false "NewEnumerator1" self)))

(event Custom|OptionalAim
  (params (Aim :type Boolean))
  ;[1 1 1] Change aim color
)

(event Collision|EventActorBeginOverlap
  (params (OtherActor :type Actor%20Object%20Reference)))

(event EventTick
  (params (DeltaSeconds :type Float%20%28single-precision%29))
  (Utilities|FlowControl|Sequence
    (:then_0
      ;[1 1 1] BarRotation
      (CallFunction|SetWidgetRotation (Variables|Default|GetBarStat)))
    (:then_1
      ;[1 1 1] FindTownCenter
      (if (Variables|Default|GetIsGhost)
        (Utilities|IsValid (Variables|Default|GetTownCenterRef)
          (:Is%20Valid
            (if (> (Math|Vector|VectorLength (- (Transformation|GetActorLocation (Variables|Default|GetTownCenterRef)) (Transformation|GetWorldLocation (Variables|Debug|GetStaticMeshComponent)))) 5e+03)
              (Variables|Default|SetTownCenterRef 0)))
          (:Is%20Not%20Valid
            (CallFunction|FindNearestTownCenter)))))))

(event EventAimActor
  (params (Aim :type Boolean) (Force :type Boolean) (InstanceIndex :type Integer) (CameraPawnRef :type Camera%20Pawn%20Object%20Reference) (ComponentAimed :type Primitive%20Component%20Object%20Reference))
  ;[1 1 1] Change aim color
  (if (or Force (not (Variables|Default|GetIsSelected)))
    (Rendering|SetCustomDepthStencilValue (Variables|Debug|GetStaticMeshComponent) (Variables|Default|GetRelation))
    (Rendering|SetRenderCustomDepth (Variables|Debug|GetStaticMeshComponent) Aim)
    (Default|ShowBar (Variables|Default|GetBarStatRef) Aim)
    (CallFunction|OptionalAim Aim)
    (if Aim
      (CallFunction|SetWidgetRotation (Variables|Default|GetBarStat)))))

(event EventSelect/UnselectActor
  (params (Select :type Boolean))
  ;[1 1 1] Select Character
  (CallFunction|AimActor Select true)
  (bind _output_get (Variables|Default|SetIsSelected Select))
  (Default|UpdatePropertiesOfTable (Variables|/Game/LowPolyProject/GameMode/StratController.StratController_C|GetStratHudRef (Variables|Default|GetControllerRef)) (not _output_get) "NewEnumerator1" self)
  (if (Variables|Default|GetIsGhost)
    _
    (else
      (CallFunction|HideRooforNot (Variables|Default|GetIsSelected))
      (Rendering|Components|Light|SetIntensity (Variables|Default|GetPointLight) (select (Variables|Default|GetIsSelected) (Variables|Default|GetLightIntensity) 0.0))))
  (Collision|SetCollisionResponsetoChannel (Variables|Debug|GetStaticMeshComponent) "ECC_GameTraceChannel1" (select (Variables|Default|GetIsSelected) "ECR_Ignore" "ECR_Block")))

(event EventBeginPlay
  (Utilities|FlowControl|Sequence
    (:then_0
      ;[1 1 1] SetControllerRef
      (bind _asstrat_controller (Utilities|Casting|CastToStratController (Game|GetPlayerController 0))
        (:then
          (Variables|Default|SetControllerRef _asstrat_controller))
        (:CastFailed
          _))
      ;[1 1 1] SetGameStateRef
      (bind _asmy_game_state (Utilities|Casting|CastToMyGameState (Game|GetGameState)))
      (Variables|Default|SetGameStateRef _asmy_game_state)
      ;[1 1 1] Add building on map
      (Utilities|IsValid (Variables|/Game/LowPolyProject/GameMode/StratController.StratController_C|GetGameInstanceRef (Variables|Default|GetControllerRef)) :!label _label
        (:Is%20Valid
          (Utilities|Map|Add (Variables|/Game/LowPolyProject/GameMode/MyGameInstance.MyGameInstance_C|GetStaticActors (Variables|/Game/LowPolyProject/GameMode/StratController.StratController_C|GetGameInstanceRef (Variables|Default|GetControllerRef))) self (Variables|Default|GetColorOnMap)))
        (:Is%20Not%20Valid
          (Utilities|FlowControl|Delay 0.2)
          (goto _label))))
    (:then_1
      ;[1 1 1] BarStatRef
      (bind _asbar_stat (Utilities|Casting|CastToBarStat (UserInterface|GetUserWidgetObject (Variables|Default|GetBarStat))))
      (bind _output_get (Variables|Default|SetBarStatRef _asbar_stat))
      (Variables|/Game/LowPolyProject/Environment/Hud/Character/BarStat.BarStat_C|SetBuildingRef _output_get self)
      ;[1 1 1] UpdateBarSize
      (Transformation|SetWorldScale3D (Variables|Default|GetBarStat) (* "1.000000,1.000000,1.000000" (/ (Variables|Default|GetBuildingWidth) 7e+01)))
      ;[1 1 1] UpdateBarState
      (Default|SetLifeBarFunction (Variables|Default|GetBarStatRef)))
    (:then_2
      ;[1 1 1] GetOriginalMaterial
      (Variables|Default|SetOriginalMaterial (Utilities|Array|Get(acopy) (Rendering|Material|GetMaterials (Variables|Debug|GetStaticMeshComponent)))))
    (:then_3
      ;[1 1 1] FlatWorld
      (Utilities|IsValid (Variables|Default|GetControllerRef)
        (:Is%20Valid
          (Default|FlatWorld (Variables|Default|GetControllerRef) (Transformation|GetActorLocation) (Variables|Default|GetBuildingWidth)))))))

(fn ConstructionScript
  ;[1 1 1] AntiBuildingRadius
  (Components|Sphere|SetSphereRadius (Variables|Default|GetSphereAntiBuilding) (Variables|Default|GetBuildingWidth) true))

(fn SetWidgetRotation
  (params (WidgetToRotate :type Scene%20Component%20Object%20Reference))
  (if (Rendering|IsVisible WidgetToRotate)
    (Transformation|SetWorldRotation WidgetToRotate (Math|Rotator|MakeRotfromX (* (Transformation|GetActorForwardVector (Game|GetPlayerCameraManager 0)) -1)) false false)))

(fn SetGhostMode
  (params (CollisionType :type ECollisionEnabled%20Enum :default "NoCollision"))
  (bind _sphereantibuilding (Variables|Default|GetSphereAntiBuilding))
  (Variables|Default|SetIsGhost (Utilities|Enum|NotEqual(Enum) CollisionType "QueryAndPhysics"))
  (for _array_element (Actor|GetComponentsbyTag "/Script/Engine.PrimitiveComponent" "Mesh")
    (Collision|SetCollisionEnabled _array_element CollisionType)
    (Collision|SetCollisionResponsetoChannel _array_element "ECC_Pawn" (select (Variables|Default|GetIsGhost) "ECR_Ignore" "ECR_Block")))
  (Collision|SetCollisionEnabled _sphereantibuilding (Utilities|Select :Index CollisionType :NoCollision "NoCollision" :QueryOnly "QueryOnly" :PhysicsOnly "PhysicsOnly" :QueryAndPhysics "QueryOnly"))
  (Collision|SetCollisionResponsetoChannel _sphereantibuilding "ECC_Pawn" (Utilities|Select :Index CollisionType :NoCollision "ECR_Ignore" :QueryOnly (select (Variables|Default|GetDoNotBlockPlayerWhenConstructed) "ECR_Ignore" "ECR_Block") :PhysicsOnly "ECR_Ignore" :QueryAndPhysics "ECR_Ignore")))

(fn HideRooforNot
  (params (Index :type Boolean))
  (if (Variables|Default|GetCanHideRoof)
    (Rendering|Material|SetMaterial (Variables|Debug|GetStaticMeshComponent) (Variables|Default|GetRoofMaterialIndex) (select Index "/Game/LowPolyProject/Environment/Materials/DecorMat/Invisible.Invisible" (Variables|Default|GetOriginalMaterial)))))

(fn FindNearestTownCenter
  (bind _staticmeshcomponent (Variables|Debug|GetStaticMeshComponent))
  (bind _returnvalue (Transformation|GetWorldLocation _staticmeshcomponent))
  (LocalVariables|SetNearestPosition 5e+03)
  (bind _outhits (Collision|MultiSphereTraceForObjects _returnvalue _returnvalue 5e+03 (Utilities|Array|MakeArray "ObjectTypeQuery7") true 0 "None"))
  (for _array_element _outhits
    (bind _astown_center_bp (Utilities|Casting|CastToTownCenterBP (.hitactor _array_element)))
    (if (< (Math|Vector|VectorLength (- (Transformation|GetActorLocation (.hitactor _array_element)) (Transformation|GetWorldLocation (Variables|Debug|GetStaticMeshComponent)))) (LocalVariables|GetNearestPosition))
      (LocalVariables|SetNearestPosition (Math|Vector|VectorLength (- (Transformation|GetActorLocation (.hitactor _array_element)) (Transformation|GetWorldLocation (Variables|Debug|GetStaticMeshComponent)))))
      (LocalVariables|SetFuturCenterRef _astown_center_bp)))
  (Variables|Default|SetTownCenterRef (LocalVariables|GetFuturCenterRef))
  (return))

(fn CreateDynamicMaterials
  (for _array_element (Actor|GetComponentsbyTag "/Script/Engine.PrimitiveComponent" "Mesh")
    (for _index (range 0 (- (Rendering|Material|GetNumMaterials _array_element) 1))
      (bind _returnvalue (Rendering|Material|CreateDynamicMaterialInstance (Rendering|Material|GetMaterial _array_element _index) "None" :!class /Script/Engine.KismetMaterialLibrary))
      (Utilities|Array|Add (Variables|Default|GetOriginalsMaterials) _returnvalue)
      (Rendering|Material|SetScalarParameterValue _returnvalue "BuildAmount" 0.0 :!class /Script/Engine.MaterialInstanceDynamic)
      (Rendering|Material|SetMaterial _array_element _index _returnvalue))))

(fn SetWidgetPositionScale
  (params (WidgetToRotate :type Scene%20Component%20Object%20Reference))
  (bind _returnvalue (Game|GetPlayerCameraManager 0))
  (bind _staticmeshcomponent (Variables|Debug|GetStaticMeshComponent))
  (bind _returnvalue_2 (Camera|GetCameraLocation _returnvalue))
  (bind _returnvalue_3 (Transformation|GetWorldLocation _staticmeshcomponent))
  (bind _returnvalue_4 (- _returnvalue_2 _returnvalue_3))
  (bind _returnvalue_5 (Math|Vector|VectorLength _returnvalue_4))
  (if (Rendering|IsVisible WidgetToRotate)
    (Transformation|SetRelativeLocation WidgetToRotate (Math|Vector|MakeVector 0.0 0.0 (Math|Float|MapRangeClamped _returnvalue_5 3e+02 4e+03 3e+02 1e+03)) false false)
    (Transformation|SetWorldScale3D WidgetToRotate (* "1.000000,1.000000,1.000000" (Math|Float|MapRangeClamped _returnvalue_5 3e+02 4e+03 0.1 1.0)))))

(fn SetWidgetOpacity
  (params (WidgetToRotate :type Widget%20Object%20Reference))
  (Widget|SetRenderOpacity WidgetToRotate (Math|Float|MapRangeClamped (Math|Vector|VectorLength (- (Camera|GetCameraLocation (Game|GetPlayerCameraManager 0)) (Transformation|GetWorldLocation (Variables|Debug|GetStaticMeshComponent)))) 3e+02 4e+03 1.0 0.1)))

(fn GetBuildLocation
  (params (OldResultHit :type Hit%20Result%20Structure))
  (bind (_bblockinghit _binitialoverlap _time _distance _location _impactpoint _normal _impactnormal _physmat _hitactor _hitcomponent _hitbonename _hititem _faceindex _tracestart _traceend) (Collision|BreakHitResult OldResultHit))
  (if (Variables|Default|GetHasSpecificBuildLocation)
    (return (Collision|MakeHitResult _bblockinghit _binitialoverlap _time _distance (+ (Variables|Default|GetSpecificBuildLocation) (Transformation|GetWorldLocation (Variables|Debug|GetStaticMeshComponent))) _impactpoint _normal _impactnormal _physmat _hitactor _hitcomponent _hitbonename _hititem _faceindex _tracestart _traceend))
    (else
      (return OldResultHit))))

(fn SetMaxAdvancement
  (for _array_element (Variables|Default|GetRessourceNeededForConstruction)
    (LocalVariables|SetFuturMaxAdvancement (+ (LocalVariables|GetFuturMaxAdvancement) (/ (Math|Conversions|ToFloat(Integer) (.ressourcealreadyget _array_element)) (Math|Conversions|ToFloat(Integer) (.ressourceneeded _array_element))))))
  (Variables|Default|SetBuildingMaxActualConstructAdvancement (Math|Float|Truncate (* (/ (LocalVariables|GetFuturMaxAdvancement) (Math|Conversions|ToFloat(Integer) (Utilities|Array|Length (Variables|Default|GetRessourceNeededForConstruction)))) (Math|Conversions|ToFloat(Integer) (Variables|Default|GetBuildingFullConstructAdvancement)))))
  (return))

(fn ShoudUpdateProperties
  (return (Variables|Default|GetIsSelected)))

(fn GetAmountNeededwithReserved
  (params (MaxAmount :type Integer) (AmountAlreadyGet :type Integer) (ReservedAmount :type Map%20of%20Character%20Object%20References%20to%20Integers))
  (LocalVariables|SetFuturAmount (- MaxAmount AmountAlreadyGet))
  (bind _values (Utilities|Map|Values ReservedAmount))
  (for _array_element _values
    (LocalVariables|SetFuturAmount (- (LocalVariables|GetFuturAmount) _array_element)))
  (return (LocalVariables|GetFuturAmount)))

(fn ReserveorFreeRessourceforBuild
  (params (Reserve :type Boolean) (AmountToReserve :type Integer) (RessourceClass :type Brut%20Ressource%20BP%20Class%20Reference) (CharacterRef :type Character%20Object%20Reference))
  (for (_array_element _array_index) (Variables|Default|GetRessourceNeededForConstruction)
    (if (== (.ressourcetype _array_element) RessourceClass)
      (LocalVariables|SetRessourceInWayTemp (.ressourceinway _array_element))
      (if Reserve
        (Utilities|Map|Add (LocalVariables|GetRessourceInWayTemp) CharacterRef AmountToReserve)
        (else
          (Utilities|Map|Remove (LocalVariables|GetRessourceInWayTemp) CharacterRef)))
      (Utilities|Struct|SetmembersinRessourcesNeededForConstruction (Utilities|Array|Get(acopy) (Variables|Default|GetRessourceNeededForConstruction) _array_index) (LocalVariables|GetRessourceInWayTemp))
      (return))))

(fn SetGhostColor
  (params (ColorChoosen :type Linear%20Color%20Structure))
  (for _array_element (Variables|Default|GetOriginalsMaterials)
    (Rendering|Material|SetVectorParameterValue _array_element "BuildColor" ColorChoosen :!class /Script/Engine.MaterialInstanceDynamic)))

(fn SetBuildAdvancement
  (params (Scalar :type Float%20%28single-precision%29))
  (for _array_element (Variables|Default|GetOriginalsMaterials)
    (Rendering|Material|SetScalarParameterValue _array_element "BuildAmount" Scalar :!class /Script/Engine.MaterialInstanceDynamic)))