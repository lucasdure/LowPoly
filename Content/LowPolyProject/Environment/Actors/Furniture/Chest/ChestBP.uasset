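; Interactable chest that, when activable, opens once and spawns a floating item for each entry in its contents.
; Opening plays a sound and two timelines that swing the cover and animate the base's rotation around its current yaw.
; If RandomContain is set, BeginPlay polls for the player pawn, gets a step from the chest's location, and adds random items from that step's ItemInChest pool, falling back to step 0.
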(event Custom|ChestOpenAnimation
  ;[1 1 1] Open Chest
  (Variables|Default|SetZRotation (.yaw (Transformation|GetWorldRotation (Variables|Default|GetStaticMeshComponent))))
  (Utilities|FlowControl|Sequence
    (:then_0
      (bind _opening (Timeline|CoverOpen PlayFromStart)
        (:Update
          (Transformation|SetRelativeRotation (Variables|Default|GetChestCover) (Math|Rotator|MakeRotator 0.0 (* _opening 1.3e+02) 0.0) false false))))
    (:then_1
      (bind _rotation (Timeline|MoveBase PlayFromStart)
        (:Update
          (Transformation|SetRelativeRotation (Variables|Default|GetStaticMeshComponent) (Math|Rotator|MakeRotator (.x _rotation) (.y _rotation) (+ (.z _rotation) (Variables|Default|GetZRotation))) false false))))))

(event EventBeginPlay
  (bind _controllerref (Variables|Default|GetControllerRef))
  (bind _playerpawnref (Variables|/Game/LowPolyProject/GameMode/StratController.StratController_C|GetPlayerPawnRef _controllerref))
  (|CallParentFunction)
  ;[1 1 1] Randomize chest container
  (if (and (Variables|Default|GetRandomContain) (Utilities|IsValid (Variables|Default|GetControllerRef)))
    (Utilities|IsValid _playerpawnref :!label _label
      (:Is%20Valid
        (CallFunction|SetRandomContent (Default|GetStepwithCoordinate _playerpawnref (Transformation|GetActorLocation))))
      (:Is%20Not%20Valid
        (Utilities|FlowControl|Delay 0.2)
        (goto _label)))))

(event Collision|EventActorBeginOverlap
  (params (OtherActor :type Actor%20Object%20Reference))
  (|CallParentFunction OtherActor) ; This node is disabled and will not be called.\nDrag off pins to build functionality.
)

(event EventTick
  (params (DeltaSeconds :type Float%20%28single-precision%29))
  (|CallParentFunction DeltaSeconds) ; This node is disabled and will not be called.\nDrag off pins to build functionality.
)

(event EventCharacterInterractwithActor
  (params (CharacterRef :type Character%20BP%20Object%20Reference))
  ;[1 1 1] Open Chest
  (if (Variables|Default|GetIsActivable)
    (CallFunction|OpenChest)))

(fn ConstructionScript
  (|CallParentFunction))

(fn OpenChest
  (if (not (Variables|Default|GetIsOpen))
    (Variables|Default|SetIsOpen true)
    (for _array_element (Variables|Default|GetChestContain)
      (bind _returnvalue (Game|SpawnActorfromClass "/Game/LowPolyProject/Environment/Actors/BrutRessource/FloatingItem/FloatingItemBP.FloatingItemBP_C" (Math|Transform|MakeTransform (Transformation|GetWorldLocation (Variables|Default|GetPositionContainer)) "0, 0, 0" "1,1,1") "AlwaysSpawn" 0 0))
      (Default|SetFloatingItem _returnvalue (.ressourceclass _array_element) (.amount _array_element) (.ressourceinit _array_element)))
    (CallFunction|ChestOpenAnimation)
    (Audio|PlaySoundatLocation "/Game/LowPolyProject/Environment/Sounds/Effect/Chest/ChestOpening.ChestOpening" (Transformation|GetActorLocation) "0, 0, 0" 1.0 1.0 0.0 0 0 0)))

(fn SetRandomContent
  (params (Step :type Integer))
  (bind _iteminchest (LocalVariables|GetItemInChest))
  (bind _value (Utilities|Map|Find _iteminchest 0))
  (bind (_value_2 _returnvalue) (Utilities|Map|Find _iteminchest Step))
  (bind _returnvalue_2 (select _returnvalue _value_2 _value))
  (for _index (range 0 (Math|Random|RandomIntegerinRange 0 3))
    (Utilities|Array|Add (Variables|Default|GetChestContain) (Utilities|Array|Get(acopy) (.itemlist _returnvalue_2) (Math|Random|RandomIntegerinRange 0 (- (Utilities|Array|Length (.itemlist _returnvalue_2)) 1))))))