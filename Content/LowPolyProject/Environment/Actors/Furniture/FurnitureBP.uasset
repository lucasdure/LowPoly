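; Base actor for furniture in the strategy game: placeable as a ghost, built with reserved resources, and selectable with a properties panel in the HUD.
; Optionally registers on the minimap, retrying until the game instance is valid.
; Aiming or selecting drives a custom-depth stencil outline and toggles the parent building's roof.
; Dynamic materials show ghost color and build progress; completion updates building and town center lists and refreshes the HUD.
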(event EventBeginPlay
  (Utilities|FlowControl|Sequence
    (:then_0
      ;[1 1 1] Get controller ref
      (bind _asstrat_controller (Utilities|Casting|CastToStratController (Game|GetPlayerController 0)))
      (bind _output_get (Variables|Default|SetControllerRef _asstrat_controller))
      ;[1 1 1] Add to map
      (if (Variables|Default|GetShouldAddOnMap)
        (Utilities|IsValid (Variables|/Game/LowPolyProject/GameMode/StratController.StratController_C|GetGameInstanceRef _output_get) :!label _label
          (:Is%20Valid
            (Utilities|Map|Add (Variables|/Game/LowPolyProject/GameMode/MyGameInstance.MyGameInstance_C|GetStaticActors (Variables|/Game/LowPolyProject/GameMode/StratController.StratController_C|GetGameInstanceRef (Variables|Default|GetControllerRef))) self (Variables|Default|GetColorOnMap))
            (Default|UpdateWidgetMiniMap (Variables|/Game/LowPolyProject/GameMode/StratController.StratController_C|GetMiniMapGenerator (Variables|Default|GetControllerRef)) true))
          (:Is%20Not%20Valid
            (Utilities|FlowControl|Delay 0.2)
            (goto _label)))))))

(event Collision|EventActorBeginOverlap
  (params (OtherActor :type Actor%20Object%20Reference)))

(event EventTick
  (params (DeltaSeconds :type Float%20%28single-precision%29)))

(event EventAimActor
  (params (Aim :type Boolean) (Force :type Boolean) (InstanceIndex :type Integer) (CameraPawnRef :type Camera%20Pawn%20Object%20Reference) (ComponentAimed :type Primitive%20Component%20Object%20Reference))
  ;[1 1 1] Aim
  (CallFunction|AimFunction Aim Force))

(event EventSelect/UnselectActor
  (params (Select :type Boolean))
  ;[1 1 1] Select Furniture
  (Utilities|IsValid (Variables|Default|GetControllerRef)
    (:Is%20Valid
      (CallFunction|AimActor Select true)
      (bind _output_get (Variables|Default|SetIsSelected Select))
      (Default|UpdatePropertiesOfTable (Variables|/Game/LowPolyProject/GameMode/StratController.StratController_C|GetStratHudRef (Variables|Default|GetControllerRef)) (not _output_get) "NewEnumerator4" self false))))

(fn ConstructionScript
  (for _array_element (Components|GetChildrenComponents (Variables|Debug|GetStaticMeshComponent) false)
    (bind _asstatic_mesh_component (Utilities|Casting|CastToStaticMeshComponent _array_element))
    (Utilities|Array|Add (Variables|Default|GetMeshToOutline) _asstatic_mesh_component))
  (Utilities|Array|Add (Variables|Default|GetMeshToOutline) (Variables|Debug|GetStaticMeshComponent)))

(fn AimFunction
  (params (Aimed :type Boolean) (Force :type Boolean))
  (Variables|Default|SetAimed Aimed)
  (if (or Force (not (Variables|Default|GetIsSelected)))
    (LocalVariables|SetOutlineColorNumber (select (Variables|Default|GetIsActivable) 1 2))
    (Utilities|IsValid (Variables|Default|GetBuildingRef)
      (:Is%20Valid
        (bind _ascharacter_bp (Utilities|Casting|CastToCharacterBP (Utilities|Array|Get(acopy) (Variables|/Game/LowPolyProject/GameMode/CameraPawn.CameraPawn_C|GetSelectedActors (Variables|/Game/LowPolyProject/GameMode/StratController.StratController_C|GetPlayerPawnRef (Variables|Default|GetControllerRef)))))
          (:then
            (LocalVariables|SetCharacterInsideBuilding (== (Variables|/Game/LowPolyProject/Environment/Actors/Characters/CharacterBP.CharacterBP_C|GetInsideBuilding _ascharacter_bp) (Variables|Default|GetBuildingRef))))
          (:CastFailed
            _))
        (Default|HideRooforNot (Variables|Default|GetBuildingRef) (Math|Boolean|ORBoolean (LocalVariables|GetCharacterInsideBuilding) (Variables|Default|GetAimed) (Variables|/Game/LowPolyProject/Environment/Actors/Building/BuildingBP.BuildingBP_C|GetIsSelected (Variables|Default|GetBuildingRef)))))
      (:Is%20Not%20Valid
        _))
    (for _array_element (Variables|Default|GetMeshToOutline)
      (Rendering|SetCustomDepthStencilValue _array_element (LocalVariables|GetOutlineColorNumber))
      (Rendering|SetRenderCustomDepth (Variables|Debug|GetStaticMeshComponent) (Variables|Default|GetAimed)))))

(fn CreateGhostMaterial
  (for _array_element (Actor|GetComponentsbyTag "/Script/Engine.PrimitiveComponent" "Mesh")
    (for _index (range 0 (- (Rendering|Material|GetNumMaterials _array_element) 1))
      (bind _returnvalue (Rendering|Material|CreateDynamicMaterialInstance (Rendering|Material|GetMaterial _array_element _index) "None" :!class /Script/Engine.KismetMaterialLibrary))
      (Utilities|Array|Add (Variables|Default|GetOriginalsMaterials) _returnvalue)
      (Rendering|Material|SetScalarParameterValue _returnvalue "BuildAmount" 0.0 :!class /Script/Engine.MaterialInstanceDynamic)
      (Rendering|Material|SetMaterial _array_element _index _returnvalue))))

(fn SetGhostColor
  (params (ColorChoosen :type Linear%20Color%20Structure))
  (for _array_element (Variables|Default|GetOriginalsMaterials)
    (Rendering|Material|SetVectorParameterValue _array_element "BuildColor" ColorChoosen :!class /Script/Engine.MaterialInstanceDynamic)))

(fn GetBuildLocation
  (params (InitialHit :type Hit%20Result%20Structure))
  (bind (_bblockinghit _binitialoverlap _time _distance _location _impactpoint _normal _impactnormal _physmat _hitactor _hitcomponent _hitbonename _hititem _faceindex _tracestart _traceend) (Collision|BreakHitResult InitialHit))
  (return (Collision|MakeHitResult _bblockinghit _binitialoverlap _time _distance (+ (Variables|Default|GetSpecificBuildLocation) (Transformation|GetWorldLocation (Variables|Debug|GetStaticMeshComponent))) _impactpoint _normal _impactnormal _physmat _hitactor _hitcomponent _hitbonename _hititem _faceindex _tracestart _traceend)))

(fn ReserveorFreeRessourceforBuild
  (params (Reserve :type Boolean) (AmountToReserve :type Integer) (RessourceClass :type Brut%20Ressource%20BP%20Class%20Reference) (CharacterRef :type Character%20BP%20Object%20Reference))
  (for (_array_element _array_index) (Variables|Default|GetRessourceNeededForConstruction)
    (if (== (.ressourcetype _array_element) RessourceClass)
      (LocalVariables|SetRessourceInWayTemp (.ressourcereserved _array_element))
      (if Reserve
        (Utilities|Map|Add (LocalVariables|GetRessourceInWayTemp) CharacterRef AmountToReserve)
        (else
          (Utilities|Map|Remove (LocalVariables|GetRessourceInWayTemp) CharacterRef)))
      (Utilities|Struct|SetmembersinRessourcesNeededForConstructionBis (Utilities|Array|Get(acopy) (Variables|Default|GetRessourceNeededForConstruction) _array_index) (LocalVariables|GetRessourceInWayTemp))
      (return))))

(fn ShouldUpdateProperties
  (return (Variables|Default|GetIsSelected)))

(fn OnConstructed
  (bind _buildingref (Variables|Default|GetBuildingRef))
  (bind _buildingref_2 (Variables|Default|GetBuildingRef))
  (bind _buildingref_3 (Variables|Default|GetBuildingRef))
  (bind _towncenterref (Variables|/Game/LowPolyProject/Environment/Actors/Building/BuildingBP.BuildingBP_C|GetTownCenterRef _buildingref_3))
  (CallFunction|SetBuildAdvancement 1.0)
  (Utilities|IsValid _buildingref_2
    (:Is%20Valid
      (Utilities|Array|Add (Variables|/Game/LowPolyProject/Environment/Actors/Building/BuildingBP.BuildingBP_C|GetFurnitureCreated _buildingref_2) self)
      (Utilities|IsValid _towncenterref
        (:Is%20Valid
          (Utilities|Array|RemoveItem (Variables|/Game/LowPolyProject/Environment/Actors/Building/BuildingBP.BuildingBP_C|GetFurnitureWaitingBuilding _towncenterref) self)
          (Utilities|Array|Add (Variables|/Game/LowPolyProject/Environment/Actors/Building/BuildingBP.BuildingBP_C|GetFurnitureCreated _towncenterref) self))
        (:Is%20Not%20Valid
          _))
      (Utilities|Array|RemoveItem (Variables|/Game/LowPolyProject/Environment/Actors/Building/BuildingBP.BuildingBP_C|GetFurnitureWaitingBuilding (Variables|Default|GetBuildingRef)) self))
    (:Is%20Not%20Valid
      _))
  (Variables|Default|SetIsGhost false)
  (if (CallFunction|ShouldUpdateProperties)
    (Default|UpdatePropertiesOfTable (Variables|/Game/LowPolyProject/GameMode/StratController.StratController_C|GetStratHudRef (Variables|Default|GetControllerRef)) false "NewEnumerator4" self true))
  (Utilities|IsValid _buildingref
    (:Is%20Valid
      (if (Default|ShouldUpdateProperties _buildingref)
        (Default|UpdatePropertiesOfTable (Variables|/Game/LowPolyProject/GameMode/StratController.StratController_C|GetStratHudRef (Variables|Default|GetControllerRef)) false "NewEnumerator1" (Variables|Default|GetBuildingRef) false)))))

(fn SetBuildAdvancement
  (params (Value :type Float%20%28single-precision%29))
  (for _array_element (Variables|Default|GetOriginalsMaterials)
    (Rendering|Material|SetScalarParameterValue _array_element "BuildAmount" Value :!class /Script/Engine.MaterialInstanceDynamic)))

(fn UpdateBuildingPropertiesBase
  (if (and (Variables|Default|GetIsSelected) (== self (Variables|/Game/LowPolyProject/Environment/Hud/Camera/StrategicHud.StrategicHud_C|GetLastValidFurniture (Variables|/Game/LowPolyProject/GameMode/StratController.StratController_C|GetStratHudRef (Variables|Default|GetControllerRef)))))
    (Utilities|IsValid (Variables|/Game/LowPolyProject/Environment/Hud/Camera/StrategicHud.StrategicHud_C|GetFurniturePropertyRef (Variables|/Game/LowPolyProject/GameMode/StratController.StratController_C|GetStratHudRef (Variables|Default|GetControllerRef)))
      (:Is%20Valid
        (if (or (Variables|Default|GetNoUsers) (Variables|Default|GetIsGhost))
          (Widget|RemovefromParent (Variables|/Game/LowPolyProject/Environment/Hud/Camera/Furniture/FurnitureProperties.FurnitureProperties_C|GetUsersButton (Variables|/Game/LowPolyProject/Environment/Hud/Camera/StrategicHud.StrategicHud_C|GetFurniturePropertyRef (Variables|/Game/LowPolyProject/GameMode/StratController.StratController_C|GetStratHudRef (Variables|Default|GetControllerRef))))))
        (if (or (Variables|Default|GetNoRessources) (Variables|Default|GetIsGhost))
          (Widget|RemovefromParent (Variables|/Game/LowPolyProject/Environment/Hud/Camera/Furniture/FurnitureProperties.FurnitureProperties_C|GetInventoryButton (Variables|/Game/LowPolyProject/Environment/Hud/Camera/StrategicHud.StrategicHud_C|GetFurniturePropertyRef (Variables|/Game/LowPolyProject/GameMode/StratController.StratController_C|GetStratHudRef (Variables|Default|GetControllerRef))))))))))