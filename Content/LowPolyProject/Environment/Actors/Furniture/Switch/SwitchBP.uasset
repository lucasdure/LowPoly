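; SwitchBP is an interactable furniture switch that toggles on and off when a character interacts with it.
; The interaction event checks IsActivable, flips IsActivated, and plays or reverses the RotateSwitch timeline to match the new state.
; The timeline's update drives the static mesh's relative pitch to animate the switch, with no other logic triggered in this graph.
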(event EventBeginPlay
  (|CallParentFunction) ; This node is disabled and will not be called.\nDrag off pins to build functionality.
)

(event Collision|EventActorBeginOverlap
  (params (OtherActor :type Actor%20Object%20Reference))
  (|CallParentFunction OtherActor) ; This node is disabled and will not be called.\nDrag off pins to build functionality.
)

(event EventTick
  (params (DeltaSeconds :type Float%20%28single-precision%29))
  (|CallParentFunction DeltaSeconds) ; This node is disabled and will not be called.\nDrag off pins to build functionality.
)

(event EventCharacterInterractwithActor
  (params (CharacterRef :type Character%20BP%20Object%20Reference))
  (if (Variables|Default|GetIsActivable)
    (if (Variables|Default|GetIsActivated)
      (Variables|Default|SetIsActivated false)
      (bind _rotation (Timeline|RotateSwitch Reverse)
        (:Update
          (Transformation|SetRelativeRotation (Variables|Default|GetStaticMesh) (Math|Rotator|MakeRotator 0.0 _rotation 0.0) false false)))
      (else
        (Variables|Default|SetIsActivated true)
        (Timeline|RotateSwitch Play)))))

(fn ConstructionScript
  (|CallParentFunction))