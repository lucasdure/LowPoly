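; Campfire camp actor that populates itself at BeginPlay with a random number of characters and furniture pieces.
; Both are placed on rings around the fire, snapped to the ground by line trace and turned toward the center.
; Units share a random skin color, start as Neutral to each other and get the campfire as their blackboard ActorToKeep.
; When the last unit is removed, the fire particles stop, furniture becomes activable and the actor destroys itself after a delay.
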(event Custom|RemoveWithDelay
  (Utilities|FlowControl|Delay 2e+01)
  (Actor|DestroyActor))

(event EventBeginPlay
  (|CallParentFunction)
  (CallFunction|SpawnRandomUnit)
  (CallFunction|SpawnRandomFurniture))

(event Collision|EventActorBeginOverlap
  (params (OtherActor :type Actor%20Object%20Reference)))

(event EventTick
  (params (DeltaSeconds :type Float%20%28single-precision%29)))

(fn ConstructionScript
  (Variables|Default|SetColorSkin (Utilities|Struct|MakeLinearColor (Math|Random|RandomFloat) (Math|Random|RandomFloat) (Math|Random|RandomFloat) 1.0)))

(fn SpawnRandomUnit
  (bind _maxminunit (Variables|Default|GetMaxMinUnit))
  (bind _output_get (LocalVariables|SetRandomValue (Math|Float|Round (Math|Float|MapRangeClamped (Math|Random|RandomFloat) 0.0 1.0 (.x _maxminunit) (.y _maxminunit)))))
  (for _index (range 0 (- _output_get 1))
    (bind _circleposition (Class|SimpleMathFunction|GetCirclePoint _index (+ _output_get 1) (Variables|Default|GetSize) (Transformation|GetWorldLocation (Variables|Default|GetStaticMeshComponent))))
    (bind _outhit (Collision|LineTraceByChannel (+ _circleposition "0, 0,1000.000000") (+ _circleposition "0, 0,-1000.000000") "TraceTypeQuery1" false 0 "None"))
    (bind _returnvalue (Game|SpawnActorfromClass (Variables|Default|GetCharacterClass) (Math|Transform|MakeTransform (.Location (Collision|BreakHitResult _outhit)) (Math|Rotator|MakeRotator 0.0 0.0 (.yaw (Math|Rotator|FindLookatRotation (.Location (Collision|BreakHitResult _outhit)) (Transformation|GetWorldLocation (Variables|Default|GetStaticMeshComponent))))) "1,1,1") "AlwaysSpawn" 0 0))
    (bind _output_get_2 (LocalVariables|SetCharacterLocal _returnvalue))
    (Variables|/Game/LowPolyProject/Environment/Actors/Characters/CharacterBP.CharacterBP_C|SetCampfire _output_get_2 self)
    (for _array_element (Variables|Default|GetUnitsInCamp)
      (Utilities|Map|Add (Variables|/Game/LowPolyProject/Environment/Actors/Characters/CharacterBP.CharacterBP_C|GetAlreadyMetCharacter (LocalVariables|GetCharacterLocal)) _array_element (Utilities|Struct|MakeMetCharacters "Neutral"))
      (Utilities|Map|Add (Variables|/Game/LowPolyProject/Environment/Actors/Characters/CharacterBP.CharacterBP_C|GetAlreadyMetCharacter _array_element) (LocalVariables|GetCharacterLocal) (Utilities|Struct|MakeMetCharacters "Neutral")))
    (Utilities|Array|Add (Variables|Default|GetUnitsInCamp) (LocalVariables|GetCharacterLocal))
    (AI|Components|Blackboard|SetValueasObject (AI|GetBlackboard (LocalVariables|GetCharacterLocal)) (Utilities|Name|MakeLiteralName "ActorToKeep") self)
    (Variables|/Game/LowPolyProject/Environment/Actors/Characters/CharacterBP.CharacterBP_C|SetSkinColor (LocalVariables|GetCharacterLocal) (Variables|Default|GetColorSkin))
    (Default|ResetSkinColor (LocalVariables|GetCharacterLocal))))

(fn CleanUnitinCamp
  (params (CharacterRef :type Character%20BP%20Object%20Reference))
  (bind _unitsincamp (Variables|Default|GetUnitsInCamp))
  (bind _returnvalue (Utilities|Array|RemoveItem _unitsincamp CharacterRef))
  (if _returnvalue
    (if (== (Utilities|Array|Length _unitsincamp) 0)
      (Effects|Components|ParticleSystem|SetFloatParameter (Variables|Default|GetParticleSystem) "SpawnNumber" 0.0)
      (for _array_element (Variables|Default|GetFurnitureCreated)
        (Variables|/Game/LowPolyProject/Environment/Actors/Furniture/FurnitureBP.FurnitureBP_C|SetIsActivable _array_element true))
      (Variables|Default|SetCampCleaned true)
      (CallFunction|RemovewithDelay))))

(fn SpawnRandomFurniture
  (bind _maxminfurniture (Variables|Default|GetMaxMinFurniture))
  (bind _furnitureclass (Variables|Default|GetFurnitureClass))
  (bind _output_get (LocalVariables|SetRandomValue (Math|Float|Round (Math|Float|MapRangeClamped (Math|Random|RandomFloat) 0.0 1.0 (.x _maxminfurniture) (.y _maxminfurniture)))))
  (for _index (range 0 (- _output_get 1))
    (bind _circleposition (Class|SimpleMathFunction|GetCirclePoint _index (+ _output_get 1) (+ (Variables|Default|GetSize) 5e+01) (Transformation|GetWorldLocation (Variables|Default|GetStaticMeshComponent))))
    (bind _outhit (Collision|LineTraceByChannel (+ _circleposition "0, 0,1000.000000") (+ _circleposition "0, 0,-1000.000000") "TraceTypeQuery1" false 0 "None"))
    (bind _returnvalue (Game|SpawnActorfromClass (Utilities|Array|Get(acopy) _furnitureclass (Math|Random|RandomIntegerinRange 0 (- (Utilities|Array|Length _furnitureclass) 1))) (Math|Transform|MakeTransform (.Location (Collision|BreakHitResult _outhit)) (Math|Rotator|MakeRotator 0.0 0.0 (.yaw (Math|Rotator|FindLookatRotation (.Location (Collision|BreakHitResult _outhit)) (Transformation|GetWorldLocation (Variables|Default|GetStaticMeshComponent))))) "1,1,1") "AlwaysSpawn" 0 0))
    (Utilities|Array|Add (Variables|Default|GetFurnitureCreated) _returnvalue)
    (Variables|/Game/LowPolyProject/Environment/Actors/Furniture/FurnitureBP.FurnitureBP_C|SetCampfireRef _returnvalue self)
    (Variables|/Game/LowPolyProject/Environment/Actors/Furniture/FurnitureBP.FurnitureBP_C|SetIsActivable _returnvalue false)))